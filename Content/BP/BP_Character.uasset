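; Player character for a turn-based, square-grid game, handling moves, Health, Clog and Luck, and game over.
; Each controller move line-traces the target square to stop, step or shovel through a block, then lights available squares.
; A timeline eases movement, mesh turn and spring-arm camera, using a row-to-pitch map built from the chunk, and triggers enemy moves.
; Forward steps raise Clog, which erodes Luck, while queued health changes apply at turn end.
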(event Custom|MoveEvent
  (params (Move :type Enum_Direction%20Enum :default "NewEnumerator0"))
  (Variables|Move|SetMoveDir Move)
  (if (Variables|/Game/BP/BP_GM.BP_GM_C|GetIsMoveFinished (Variables|Ref|GetGameMode_Ref))
    (Variables|/Game/BP/BP_GM.BP_GM_C|SetIsMoveFinished (Variables|Ref|GetGameMode_Ref) false)
    (CallFunction|SetCharStatusOldVariables) ; Clog, Health etc. before Move
    (bind _state (Move|LineTrace|LTIsThereSquare 1.0))
    (switch Utilities|FlowControl|Switch|SwitchonEnum_CharacterStates _state
      (:NewEnumerator7
        (Default|LineCollisionFollowCharacter (Variables|Ref|GetGreyLine_Ref) :!label _label)
        (Move|LineTrace|LTLightAvailableSquares :!label _label_2)
        (Variables|/Game/BP/BP_GM.BP_GM_C|SetIsMoveFinished (Variables|Ref|GetGameMode_Ref) true)
        (bind _is_health_0 (Status|Health|DoChangeHealth))
        (CallFunction|CreateGameOverWidget _is_health_0))
      (:NewEnumerator4
        (goto _label))
      (:NewEnumerator5
        (goto _label_2))
      (:NewEnumerator0
        (|Timeline|Lerp|SetActorLocation :!label _label_3
          (:Finished
            (goto _label))
          (:Before%20Timeline
            (Default|CallEnemyMove _state)
            (Utilities|MoveForwardCounter (Variables|Move|GetMoveDir)))))
      (:NewEnumerator2
        (Status|Clog|ChangeClog 1 :!label _label_4)
        (Status|ClogtoLuck)
        (goto _label_3))
      (:NewEnumerator3
        (goto _label_4))
      (:NewEnumerator6
        (Class|InterfaceDestroyable|Destroyable(Message) (Variables|Move|IsThereSquare|GetHitActor_Move))
        (Variables|/Game/BP/BP_GM.BP_GM_C|SetIsShovelActive (Variables|Ref|GetGameMode_Ref) false)
        (Status|ClogtoLuck)
        (goto _label_3)))))

(event EventBeginPlay
  (Ref|SetPlayerControllerRef)
  (Ref|SetGameModeRef)
  (Ref|SetChunkRef)
  (Ref|SetGreyLineRef)
  (EventDispatchers|AssignMoveEvent (Variables|Ref|GetPlayerController_Ref) (EventDispatchers|CreateEvent :!event Custom|MoveEvent))
  (bind _returnvalue (UserInterface|CreateWidget "/Game/BP/UI/UI_InGame.UI_InGame_C"))
  (UserInterface|Viewport|AddtoViewport _returnvalue 0)
  (CameraOffset(SpringArm)|DoMapCameraLocYtoRotY -1.0)
  (Utilities|FlowControl|Delay 0.0)
  (Transformation|AddActorWorldOffset "250.000000, 0, 0")
  (Rendering|SetVisibility (Variables|Character|GetMesh) true false)
  (Variables|/Game/BP/BP_GM.BP_GM_C|SetIsMoveFinished (Variables|Ref|GetGameMode_Ref) true)
  (Move|LineTrace|LTLightAvailableSquares))

(event EventTick
  (params (DeltaSeconds :type Float%20%28single-precision%29))
  (Variables|Default|SetDelta DeltaSeconds))

(fn ConstructionScript)

(fn SetPlayerControllerRef
  (Utilities|IsValid (Variables|Ref|GetPlayerController_Ref)
    (:Is%20Not%20Valid
      (bind _returnvalue (Actor|GetActorOfClass "/Game/BP/BP_PlayerController.BP_PlayerController_C"))
      (Variables|Ref|SetPlayerController_Ref _returnvalue))))

(fn LTIsThereSquare
  (params (Camera%20Rotation%20Z%20Offset%20Coefficient :type Float%20%28double-precision%29))
  ;[0.09375 0.09375 0.09375] Set Location Variables
  (Variables|Move|IsthereSquare|SetMove_Location_Old (Transformation|GetActorLocation))
  (Variables|Move|IsThereSquare|SetMove_Location_New (+ (Transformation|GetActorLocation) (Utilities|Array|Get(acopy) (Variables|Move|IsThereSquare|Get3_Turns) (Utilities|Select :Index (Variables|Move|GetMoveDir) :NewEnumerator0 0 :NewEnumerator1 1 :NewEnumerator2 2 :NewEnumerator3 3))))
  (CameraOffset(SpringArm)|CameraOffsetVariablesSetting Camera%20Rotation%20Z%20Offset%20Coefficient)
  ;[0.09375 0.09375 0.09375] Shoot a Ray
  (bind (_outhit _returnvalue) (Collision|LineTraceForObjects (+ "0,0,300.000000" (Variables|Move|IsthereSquare|GetMove_Location_Old)) (+ "0,0,-100.000000" (Variables|Move|IsThereSquare|GetMove_Location_New)) (LocalVariables|GetObjectTypes_Local) false 0 "None" true "(R=1.000000,G=0.434030,B=0.000000,A=1.000000)" "(R=0.000000,G=1.000000,B=0.000000,A=1.000000)" 1.0))
  (bind _output_get (LocalVariables|SetisHit? _returnvalue))
  (if _output_get ; is Hit?
    (Variables|Move|IsThereSquare|SetHitActor_Move (.HitActor (Collision|BreakHitResult _outhit)))
    (if (Move|Condition|IsBlockSquare) ; is Block?
      (if (Move|Condition|IsForward) ; is Forward?
        (if (Move|Condition|IsShovel) ; is Shovel?
          (return "NewEnumerator6")
          (else
            (return "NewEnumerator5")))
        (else
          (return "NewEnumerator4")))
      (elif (Move|Condition|IsForward) ; is Forward?
        (if (Move|Condition|IsShovel) ; is Shovel?
          (return "NewEnumerator3")
          (else
            (return "NewEnumerator2")))
        (else
          (return "NewEnumerator0"))))
    (else
      (return "NewEnumerator7"))))

(fn LTLightAvailableSquares
  (bind _array_element (Utilities|Array|ForEachLoopwithBreak (Variables|Move|IsThereSquare|Get3_Turns))
    (:LoopBody
      (bind (_outhit _returnvalue) (Collision|LineTraceForObjects (+ "0,0,300.000000" (Transformation|GetActorLocation)) (+ "0,0,-100.000000" (+ _array_element (Transformation|GetActorLocation))) (LocalVariables|GetObjectTypes_Local) false 0 "None" true "(R=1.000000,G=0.434030,B=0.000000,A=1.000000)" "(R=0.000000,G=1.000000,B=0.000000,A=1.000000)" 1.0))
      (if _returnvalue
        (Class|InterfaceLightSquares|LightSquare(Message) (.HitActor (Collision|BreakHitResult _outhit)))))))

(fn SetGameModeRef
  (Utilities|IsValid (Variables|Ref|GetGameMode_Ref)
    (:Is%20Not%20Valid
      (bind _asbp_gm (Utilities|Casting|CastToBP_GM (Game|GetGameMode)))
      (Variables|Ref|SetGameMode_Ref _asbp_gm))))

(fn WriteChangeHealth
  (params (Damage :type Integer))
  (Utilities|Array|Add (Variables|Status|Health|GetHealth_OverTurnArray) Damage))

(fn ChangeLuck
  (params (Luck%20Coef :type Integer))
  (Variables|Status|Luck|SetChar_Luck (Math|Integer|Clamp(Integer) (+ Luck%20Coef (Variables|Status|Luck|GetChar_Luck)) 0 10)))

(fn ChangeClog
  (params (Clog%20Coef :type Integer))
  (bind _output_get (Variables|Status|Clog|SetChar_Clog (Math|Integer|Clamp(Integer) (+ Clog%20Coef (Variables|Status|Clog|GetChar_Clog)) 0 100)))
  (Variables|Status|Clog|SetClogAmount_New _output_get)
  (Variables|Status|Clog|SetClogAmount_Differ (Math|Integer|Absolute(Integer) (- (Variables|Status|Clog|GetClogAmount_Old) (Variables|Status|Clog|GetClogAmount_New)))))

(fn IsBlockSquare
  (return (or (== (Utilities|GetClass (Variables|Move|IsThereSquare|GetHitActor_Move)) "/Game/BP/BP_Square_Block.BP_Square_Block_C") (Utilities|ClassIsChildOf (Utilities|GetClass (Variables|Move|IsThereSquare|GetHitActor_Move)) "/Game/BP/BP_Square_Block.BP_Square_Block_C"))))

(fn IsForward
  (return (Utilities|Enum|Equal(Enum) (Variables|Move|GetMoveDir) "NewEnumerator1")))

(fn IsShovel
  (return (Variables|/Game/BP/BP_GM.BP_GM_C|GetIsShovelActive (Variables|Ref|GetGameMode_Ref))))

(fn CallOffsetChunk|ChangeClog
  (params (Clog%20Coef :type Integer))
  (Default|CallOffsetChunk)
  (Status|Clog|ChangeClog Clog%20Coef))

(fn CameraOffsetonMove
  (params (Alpha :type Float%20%28double-precision%29))
  (bind _springarm (Variables|Default|GetSpringArm))
  (bind _camerarotation_old (Variables|CameraOffset|GetCameraRotation_Old))
  (bind _camerarotation_new (Variables|CameraOffset|GetCameraRotation_New))
  (bind _result (Math|Interpolation|Ease "EaseInOut" Alpha _camerarotation_old _camerarotation_new true 1.0))
  (bind _relativelocation (Variables|/Script/Engine.SceneComponent|GetRelativeLocation _springarm))
  (Transformation|SetRelativeLocation (Variables|Default|GetSpringArm) (Math|Vector|MakeVector (.x _relativelocation) (.y (Math|Interpolation|Ease "EaseInOut" Alpha (Variables|CameraOffset|GetCameraLocation_Old) (Variables|CameraOffset|GetCameraLocation_New) 3.0)) (.z _relativelocation)) false false)
  (Transformation|SetRelativeRotation (Variables|Default|GetSpringArm) (Math|Rotator|MakeRotator (.roll (Variables|/Script/Engine.SceneComponent|GetRelativeRotation (Variables|Default|GetSpringArm))) (.pitch _result) (.yaw _result)) false false))

(fn CameraOffsetVariablesSetting
  (params (Camera%20Rotation%20Z%20Offset%20Coefficient :type Float%20%28double-precision%29))
  (bind _springarm (Variables|Default|GetSpringArm))
  (bind _springarm_2 (Variables|Default|GetSpringArm))
  (bind _move_location_new (Variables|Move|IsThereSquare|GetMove_Location_New))
  (bind _move_location_new_2 (Variables|Move|IsThereSquare|GetMove_Location_New))
  (bind _springarm_3 (Variables|Default|GetSpringArm))
  (bind _springarm_4 (Variables|Default|GetSpringArm))
  (bind _cameralocytoroty (Variables|CameraOffset|GetCameraLocYtoRotY))
  (bind _cameralocytoroty_2 (Variables|CameraOffset|GetCameraLocYtoRotY))
  (bind _returnvalue (Math|Float|Round (.y _move_location_new_2)))
  (bind _returnvalue_2 (Math|Float|Round (.y _move_location_new)))
  (bind _relativerotation (Variables|/Script/Engine.SceneComponent|GetRelativeRotation _springarm_2))
  (bind _relativerotation_2 (Variables|/Script/Engine.SceneComponent|GetRelativeRotation _springarm_3))
  (bind _relativerotation_3 (Variables|/Script/Engine.SceneComponent|GetRelativeRotation _springarm_4))
  (bind _relativelocation (Variables|/Script/Engine.SceneComponent|GetRelativeLocation _springarm))
  (bind (_value _returnvalue_3) (Utilities|Map|Find _cameralocytoroty_2 _returnvalue))
  (bind (_value_2 _returnvalue_4) (Utilities|Map|Find _cameralocytoroty _returnvalue_2))
  (LocalVariables|SetRot%20Z%20Offset%20Coef Camera%20Rotation%20Z%20Offset%20Coefficient)
  (Variables|CameraOffset|SetCameraLocation_Old (Variables|/Script/Engine.SceneComponent|GetRelativeLocation (Variables|Default|GetSpringArm)))
  (Variables|CameraOffset|SetCameraLocation_New (Math|Vector|MakeVector (.x _relativelocation) (- (.y _relativelocation) (/ (.y (Utilities|Array|Get(acopy) (Variables|Move|IsThereSquare|Get3_Turns) (Utilities|Select :Index (Variables|Move|GetMoveDir) :NewEnumerator0 0 :NewEnumerator1 1 :NewEnumerator2 2 :NewEnumerator3 3))) 2.0)) (.z _relativelocation)))
  (Variables|CameraOffset|SetCameraRotation_Old (Variables|/Script/Engine.SceneComponent|GetRelativeRotation (Variables|Default|GetSpringArm)))
  (switch int (Utilities|Select :Index (Variables|Move|GetMoveDir) :NewEnumerator0 0 :NewEnumerator1 1 :NewEnumerator2 2 :NewEnumerator3 3)
    (:0
      (if _returnvalue_4
        (Variables|CameraOffset|SetCameraRotation_New (Math|Rotator|MakeRotator (.roll _relativerotation_2) _value_2 (- (.yaw _relativerotation_2) (LocalVariables|GetRot%20Z%20Offset%20Coef))))))
    (:1
      (Variables|CameraOffset|SetCameraRotation_New (Math|Rotator|MakeRotator (.roll _relativerotation) (.pitch _relativerotation) (.yaw _relativerotation))))
    (:2
      (if _returnvalue_3
        (Variables|CameraOffset|SetCameraRotation_New (Math|Rotator|MakeRotator (.roll _relativerotation_3) _value (+ (.yaw _relativerotation_3) (LocalVariables|GetRot%20Z%20Offset%20Coef))))))))

(fn DoMapCameraLocYtoRotY
  (params (Camera%20Y%20Rotation%20Coefficient :type Float%20%28double-precision%29))
  (bind _chunk_ref (Variables|Ref|GetChunk_Ref))
  (LocalVariables|SetRot%20Coef Camera%20Y%20Rotation%20Coefficient)
  (Utilities|Map|Clear (Variables|CameraOffset|GetCameraLocYtoRotY))
  (LocalVariables|SetCenter (Math|Float|Truncate (* (/ (Math|Conversions|ToFloat(Integer) (Variables|/Game/BP/BP_Chunk.BP_Chunk_C|GetAmount%20Rows%20Y _chunk_ref)) 2.0) (Math|Conversions|ToFloat(Integer) (Variables|/Game/BP/BP_Chunk.BP_Chunk_C|GetSizeOffset _chunk_ref)))))
  (Utilities|FlowControl|Sequence
    (:then_0
      (bind _index (Utilities|FlowControl|ForLoopwithBreak 0 (/ (Variables|/Game/BP/BP_Chunk.BP_Chunk_C|GetAmount%20Rows%20Y (Variables|Ref|GetChunk_Ref)) 2))
        (:LoopBody
          (Utilities|Map|Add (Variables|CameraOffset|GetCameraLocYtoRotY) (- (LocalVariables|GetCenter) (* _index (Variables|/Game/BP/BP_Chunk.BP_Chunk_C|GetSizeOffset (Variables|Ref|GetChunk_Ref)))) (+ (* _index (LocalVariables|GetRot%20Coef)) (LocalVariables|GetRotY%20Center))))
        (:Completed
          ;[0.06771 0.06771 0.06771] Reverse first map fullfilment
          (Utilities|Array|Clear (LocalVariables|GetKeys_Local))
          (bind _keys (Utilities|Map|Keys (Variables|CameraOffset|GetCameraLocYtoRotY)))
          (bind _arrayelement (Utilities|Array|ReverseforEachLoop _keys)
            (:LoopBody
              (Utilities|Array|Add (LocalVariables|GetKeys_Local) _arrayelement))
            (:Completed
              (Utilities|Array|Clear (LocalVariables|GetValues_Local))
              (bind _values (Utilities|Map|Values (Variables|CameraOffset|GetCameraLocYtoRotY)))
              (bind _arrayelement_2 (Utilities|Array|ReverseforEachLoop _values)
                (:LoopBody
                  (Utilities|Array|Add (LocalVariables|GetValues_Local) _arrayelement_2))
                (:Completed
                  (Utilities|Map|Clear (Variables|CameraOffset|GetCameraLocYtoRotY))
                  (for _index_2 (range 0 (Utilities|Array|LastIndex (LocalVariables|GetKeys_Local)))
                    (Utilities|Map|Add (Variables|CameraOffset|GetCameraLocYtoRotY) (Utilities|Array|Get(acopy) (LocalVariables|GetKeys_Local) _index_2) (Utilities|Array|Get(acopy) (LocalVariables|GetValues_Local) _index_2))))))))))
    (:then_1
      (Utilities|Map|Add (Variables|CameraOffset|GetCameraLocYtoRotY) (LocalVariables|GetCenter) (LocalVariables|GetRotY%20Center)))
    (:then_2
      (bind _index_3 (Utilities|FlowControl|ForLoopwithBreak 0 (/ (Variables|/Game/BP/BP_Chunk.BP_Chunk_C|GetAmount%20Rows%20Y (Variables|Ref|GetChunk_Ref)) 2))
        (:LoopBody
          (Utilities|Map|Add (Variables|CameraOffset|GetCameraLocYtoRotY) (+ (* _index_3 (Variables|/Game/BP/BP_Chunk.BP_Chunk_C|GetSizeOffset (Variables|Ref|GetChunk_Ref))) (LocalVariables|GetCenter)) (+ (* _index_3 (LocalVariables|GetRot%20Coef)) (LocalVariables|GetRotY%20Center))))))))

(fn SetChunkRef
  (Utilities|IsValid (Variables|Ref|GetChunk_Ref)
    (:Is%20Not%20Valid
      (bind _returnvalue (Actor|GetActorOfClass "/Game/BP/BP_Chunk.BP_Chunk_C"))
      (Variables|Ref|SetChunk_Ref _returnvalue))))

(fn SetGreyLineRef
  (Utilities|IsValid (Variables|Ref|GetGreyLine_Ref)
    (:Is%20Not%20Valid
      (bind _returnvalue (Actor|GetActorOfClass "/Game/BP/BP_GreyLine.BP_GreyLine_C"))
      (Variables|Ref|SetGreyLine_Ref _returnvalue))))

(fn ClogtoLuck
  (Variables|Status|Clog|SetClogAmount_New (Variables|Status|Clog|GetChar_Clog))
  (Variables|Status|Clog|ClogtoLuck|SetClog%2819%29Counter (+ (Math|Integer|Absolute(Integer) (- (Variables|Status|Clog|GetClogAmount_Old) (Variables|Status|Clog|GetClogAmount_New))) (Variables|Status|Clog|ClogtoLuck|GetClog%2819%29Counter)))
  (if (>= (Variables|Status|Clog|GetChar_Clog) 90)
    (if (Math|Random|RandomBoolwithWeight 0.3)
      (Status|Luck|ChangeLuck -1)
      (if (>= (Variables|Status|Clog|ClogtoLuck|GetClog%2819%29Counter) 19) :!label _label
        (Variables|Status|Clog|ClogtoLuck|SetClog%2819%29Counter 0) ; reset counter
        (Status|Luck|ChangeLuck -1)
        (Default|CheckLuckChangeChancesMap (Variables|Ref|GetGameMode_Ref))))
    (else
      (goto _label))))

(fn SetCharStatusOldVariables
  (Utilities|Array|Clear (Variables|Status|Health|GetHealth_OverTurnArray))
  (Variables|Status|Health|SetHealth_OverTurn 0)
  (Variables|Status|Health|SetHealthAmount_Old (Variables|Status|Health|GetChar_Health))
  (Variables|Status|Clog|SetClogAmount_Old (Variables|Status|Clog|GetChar_Clog)))

(fn SpawnFlyingText
  (if (!= (Variables|Status|Health|GetHealth_OverTurn) 0)
    (Game|SpawnActorfromClass "/Game/BP/BP_FlyingStatusText.BP_FlyingStatusText_C" (Math|Transform|MakeTransform (Transformation|GetActorLocation) "0, 0, 0" "1.000000,1.000000,1.000000") "AdjustIfPossibleButAlwaysSpawn" 0 0)))

(fn DoChangeHealth
  (for _array_element (Variables|Status|Health|GetHealth_OverTurnArray)
    (Variables|Status|Health|SetHealth_OverTurn (+ _array_element (Variables|Status|Health|GetHealth_OverTurn))))
  (Variables|Status|Health|SetChar_Health (Math|Integer|Clamp(Integer) (+ (Variables|Status|Health|GetHealth_OverTurn) (Variables|Status|Health|GetChar_Health)) 0 100))
  (CallFunction|SpawnFlyingText)
  (return (<= (Variables|Status|Health|GetChar_Health) 0)))

(fn CreateGameOverWidget
  (params (is%20Health%200 :type Boolean))
  (if is%20Health%200
    (Variables|/Game/BP/BP_GM.BP_GM_C|SetIsMoveFinished (Variables|Ref|GetGameMode_Ref) false)
    (Variables|Move|SetMoveForward_CounterFlag false)
    (bind _foundwidgets (Widget|GetAllWidgetsOfClass "/Game/BP/UI/UI_InGame.UI_InGame_C" true))
    (for _array_element _foundwidgets
      (Utilities|IsValid _array_element
        (:Is%20Valid
          (Widget|RemovefromParent _array_element))))
    (bind _returnvalue (UserInterface|CreateWidget "/Game/BP/UI/UI_GameOver.UI_GameOver_C" (Variables|Ref|GetPlayerController_Ref)))
    (UserInterface|Viewport|AddtoViewport _returnvalue 0))
  (return))

(fn Destroyable)