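; BP_GreyLine is an actor with a box collision line sized to span the rows of BP_Chunk along Y.
; On BeginPlay it caches the character, chunk and player controller, then after a short delay sizes and offsets LineCollision from the chunk's tile size and row count.
; It binds to the controller's move event, but that handler and the overlap handler are empty.
; A function to trail a target along X exists but is never called here.
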(event OnComponentBeginOverlap(LineCollision)
  (params (OverlappedComponent :type Primitive%20Component%20Object%20Reference) (OtherActor :type Actor%20Object%20Reference) (OtherComp :type Primitive%20Component%20Object%20Reference) (OtherBodyIndex :type Integer) (bFromSweep :type Boolean) (SweepResult :type Hit%20Result%20Structure%20%28by%20ref%29)))

(event Custom|MoveEvent
  (params (Move :type Enum_Direction%20Enum :default "NewEnumerator0")))

(event EventBeginPlay
  (Ref|SetCharacterRef)
  (Ref|SetChunkRef)
  (Ref|SetPlayerControllerRef)
  (EventDispatchers|AssignMoveEvent (Variables|Ref|GetPlayerController_Ref) (EventDispatchers|CreateEvent :!event Custom|MoveEvent))
  (Utilities|FlowControl|Delay 0.1)
  (Setup|SetSizeandPostionOfLineCollision))

(event EventTick
  (params (DeltaSeconds :type Float%20%28single-precision%29)))

(fn ConstructionScript)

(fn SetChunkRef
  (Utilities|IsValid (Variables|Ref|GetChunk_Ref)
    (:Is%20Not%20Valid
      (bind _returnvalue (Actor|GetActorOfClass "/Game/BP/BP_Chunk.BP_Chunk_C"))
      (Variables|Ref|SetChunk_Ref _returnvalue))))

(fn SetCharacterRef
  (Utilities|IsValid (Variables|Ref|GetCharacter_Ref)
    (:Is%20Not%20Valid
      (bind _returnvalue (Actor|GetActorOfClass "/Game/BP/BP_Character.BP_Character_C"))
      (Variables|Ref|SetCharacter_Ref _returnvalue))))

(fn SetPlayerControllerRef
  (Utilities|IsValid (Variables|Ref|GetPlayerController_Ref)
    (:Is%20Not%20Valid
      (bind _returnvalue (Actor|GetActorOfClass "/Game/BP/BP_PlayerController.BP_PlayerController_C"))
      (Variables|Ref|SetPlayerController_Ref _returnvalue))))

(fn SetSizeandPostionOfLineCollision
  (bind _linecollision (Variables|Default|GetLineCollision))
  (bind _chunk_ref (Variables|Ref|GetChunk_Ref))
  (bind _chunk_ref_2 (Variables|Ref|GetChunk_Ref))
  (bind _returnvalue (Transformation|GetWorldLocation _linecollision))
  (Components|Box|SetBoxExtent (Variables|Default|GetLineCollision) (Math|Vector|MakeVector (Math|Conversions|ToFloat(Integer) (/ (Variables|/Game/BP/BP_Chunk.BP_Chunk_C|GetSizeOffset (Variables|Ref|GetChunk_Ref)) 4)) (/ (* (Variables|/Game/BP/BP_Chunk.BP_Chunk_C|GetSizeOffset _chunk_ref) (Variables|/Game/BP/BP_Chunk.BP_Chunk_C|GetAmount%20Rows%20Y _chunk_ref)) 2) 5e+01) true)
  (Transformation|SetWorldLocation (Variables|Default|GetLineCollision) (Math|Vector|MakeVector (+ (/ (Variables|/Game/BP/BP_Chunk.BP_Chunk_C|GetSizeOffset (Variables|Ref|GetChunk_Ref)) 4) (.x _returnvalue)) (+ (.y _returnvalue) (/ (* (Variables|/Game/BP/BP_Chunk.BP_Chunk_C|GetSizeOffset _chunk_ref_2) (Variables|/Game/BP/BP_Chunk.BP_Chunk_C|GetAmount%20Rows%20Y _chunk_ref_2)) 2)) 0.0) false false))

(fn LineCollisionFollowCharacter
  (params (Target :type Actor%20Object%20Reference))
  (bind _returnvalue (Transformation|GetActorLocation))
  (Transformation|SetActorLocation (Math|Vector|MakeVector (- (.x (Transformation|GetActorLocation Target)) 5e+01) (.y _returnvalue) (.z _returnvalue)) false true))