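; AI enemy character that hops across a grid of squares, picking left, forward or right at random.
; BeginPlay caches references, places it by the chunk and starts a looping timer.
; Each move line-traces the target square, branches on block, forward and shovel state, then eases position and yaw via timeline.
; Moves update clog, which erodes luck; queued health changes spawn flying text and open game over at zero.
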(event Custom|MoveAICharacter
  (Variables|Move|SetMoveDir (Utilities|Select :Index (Math|Random|RandomIntegerinRange 0 2) :Option%200 "NewEnumerator0" :Option%201 "NewEnumerator1" :Option%202 "NewEnumerator2"))
  (if (Variables|/Game/BP/BP_GM.BP_GM_C|GetIsAICharMoveFin (Variables|Ref|GetGameMode_Ref))
    (Variables|/Game/BP/BP_GM.BP_GM_C|SetIsAICharMoveFin (Variables|Ref|GetGameMode_Ref) false)
    (CallFunction|SetCharStatusOldVariables) ; Clog, Health etc. before Move
    (bind _state (Move|LineTrace|LTIsThereSquare))
    (bind _output_get (Variables|Move|SetCharStates _state))
    (switch Utilities|FlowControl|Switch|SwitchonEnum_CharacterStates _output_get
      (:NewEnumerator7
        (Default|LineCollisionFollowCharacter (Variables|Ref|GetGreyLine_Ref) :!label _label)
        (Move|LineTrace|LTLightAvailableSquares :!label _label_2)
        (Variables|/Game/BP/BP_GM.BP_GM_C|SetIsAICharMoveFin (Variables|Ref|GetGameMode_Ref) true)
        (bind _is_health_0 (Status|Health|DoChangeHealth))
        (CallFunction|CreateGameOverWidget _is_health_0))
      (:NewEnumerator4
        (goto _label))
      (:NewEnumerator5
        (goto _label_2))
      (:NewEnumerator0
        (|Timeline|Lerp|SetActorLocation :!label _label_3
          (:Finished
            (goto _label))
          (:Before%20Timeline
            (Default|CallEnemyMove (Variables|Move|GetCharStates))
            (Utilities|MoveForwardCounter (Variables|Move|GetMoveDir)))))
      (:NewEnumerator2
        (Status|Clog|ChangeClog 1 :!label _label_4)
        (Status|ClogtoLuck)
        (goto _label_3))
      (:NewEnumerator3
        (goto _label_4))
      (:NewEnumerator6
        (Class|BPIDestroyable|Destroyable(Message) (Variables|Move|IsThereSquare|GetHitActor_Move))
        (Variables|/Game/BP/BP_GM.BP_GM_C|SetIsShovelActive (Variables|Ref|GetGameMode_Ref) false)
        (Status|ClogtoLuck)
        (goto _label_3)))))

(event EventBeginPlay
  (bind _returnvalue (Transformation|GetActorLocation))
  (Ref|SetPlayerControllerRef)
  (Ref|SetGameModeRef)
  (Ref|SetChunkRef)
  (Ref|SetGreyLineRef)
  (bind _returnvalue_2 (UserInterface|CreateWidget "/Game/BP/UI/UI_InGame.UI_InGame_C"))
  (UserInterface|Viewport|AddtoViewport _returnvalue_2 0)
  (Utilities|FlowControl|Delay 0.0)
  (Transformation|SetActorLocation (Math|Vector|MakeVector (.x _returnvalue) (+ (Default|FindCenterY (Variables|Ref|GetChunk_Ref)) 5.5e+02) (.z _returnvalue)) false true)
  (Transformation|AddActorWorldOffset "250.0,0.0,0.0" false true)
  (Rendering|SetVisibility (Variables|Character|GetMesh) true false)
  (Variables|/Game/BP/BP_GM.BP_GM_C|SetIsAICharMoveFin (Variables|Ref|GetGameMode_Ref) true)
  (Move|LineTrace|LTLightAvailableSquares)
  (Utilities|FlowControl|Delay 3.0)
  (Utilities|Time|SetTimerbyEvent (EventDispatchers|CreateEvent :!event Custom|MoveAICharacter) 0.35 true))

(event EventTick
  (params (DeltaSeconds :type Float%20%28single-precision%29))
  (Variables|Default|SetDelta DeltaSeconds))

(fn ConstructionScript)

(fn SetPlayerControllerRef
  (Utilities|IsValid (Variables|Ref|GetPlayerController_Ref)
    (:Is%20Not%20Valid
      (bind _returnvalue (Actor|GetActorOfClass "/Game/BP/BP_PlayerController.BP_PlayerController_C"))
      (Variables|Ref|SetPlayerController_Ref _returnvalue))))

(fn LTIsThereSquare
  ;[0.09375 0.09375 0.09375] Set Location Variables
  (Variables|Move|IsthereSquare|SetMove_Location_Old (Transformation|GetActorLocation))
  (Variables|Move|IsThereSquare|SetMove_Location_New (+ (Transformation|GetActorLocation) (Utilities|Array|Get(acopy) (Variables|Move|IsThereSquare|Get3_Turns) (Utilities|Select :Index (Variables|Move|GetMoveDir) :NewEnumerator0 0 :NewEnumerator1 1 :NewEnumerator2 2 :NewEnumerator3 3))))
  ;[0.09375 0.09375 0.09375] Shoot a Ray
  (bind (_outhit _returnvalue) (Collision|LineTraceForObjects (+ "0,0,300.000000" (Variables|Move|IsthereSquare|GetMove_Location_Old)) (+ "0,0,-100.000000" (Variables|Move|IsThereSquare|GetMove_Location_New)) (LocalVariables|GetObjectTypes_Local) false 0 "None" true "(R=1.000000,G=0.434030,B=0.000000,A=1.000000)" "(R=0.000000,G=1.000000,B=0.000000,A=1.000000)" 1.0))
  (bind _output_get (LocalVariables|SetisHit? _returnvalue))
  (if _output_get ; is Hit?
    (Variables|Move|IsThereSquare|SetHitActor_Move (.HitActor (Collision|BreakHitResult _outhit)))
    (if (Move|Condition|IsBlockSquare) ; is Block?
      (if (Move|Condition|IsForward) ; is Forward?
        (if (Move|Condition|IsShovel) ; is Shovel?
          (return "NewEnumerator6")
          (else
            (return "NewEnumerator5")))
        (else
          (return "NewEnumerator4")))
      (elif (Move|Condition|IsForward) ; is Forward?
        (if (Move|Condition|IsShovel) ; is Shovel?
          (return "NewEnumerator3")
          (else
            (return "NewEnumerator2")))
        (else
          (return "NewEnumerator0"))))
    (else
      (return "NewEnumerator7"))))

(fn LTLightAvailableSquares
  (bind _array_element (Utilities|Array|ForEachLoopwithBreak (Variables|Move|IsThereSquare|Get3_Turns))
    (:LoopBody
      (bind (_outhit _returnvalue) (Collision|LineTraceForObjects (+ "0,0,300.000000" (Transformation|GetActorLocation)) (+ "0,0,-100.000000" (+ _array_element (Transformation|GetActorLocation))) (LocalVariables|GetObjectTypes_Local) false 0 "None" true "(R=1.000000,G=0.434030,B=0.000000,A=1.000000)" "(R=0.000000,G=1.000000,B=0.000000,A=1.000000)" 1.0))
      (if _returnvalue
        (Class|BPILightSquares|LightSquare(Message) (.HitActor (Collision|BreakHitResult _outhit)))))))

(fn SetGameModeRef
  (Utilities|IsValid (Variables|Ref|GetGameMode_Ref)
    (:Is%20Not%20Valid
      (bind _asbp_gm (Utilities|Casting|CastToBP_GM (Game|GetGameMode)))
      (Variables|Ref|SetGameMode_Ref _asbp_gm))))

(fn WriteChangeHealth
  (params (Damage :type Integer))
  (Utilities|Array|Add (Variables|Status|Health|GetHealth_OverTurnArray) Damage))

(fn ChangeLuck
  (params (Luck%20Coef :type Integer))
  (Variables|Status|Luck|SetChar_Luck (Math|Integer|Clamp(Integer) (+ Luck%20Coef (Variables|Status|Luck|GetChar_Luck)) 0 10)))

(fn ChangeClog
  (params (Clog%20Coef :type Integer))
  (bind _output_get (Variables|Status|Clog|SetChar_Clog (Math|Integer|Clamp(Integer) (+ Clog%20Coef (Variables|Status|Clog|GetChar_Clog)) 0 100)))
  (Variables|Status|Clog|SetClogAmount_New _output_get)
  (Variables|Status|Clog|SetClogAmount_Differ (Math|Integer|Absolute(Integer) (- (Variables|Status|Clog|GetClogAmount_Old) (Variables|Status|Clog|GetClogAmount_New)))))

(fn IsBlockSquare
  (return (or (== (Utilities|GetClass (Variables|Move|IsThereSquare|GetHitActor_Move)) "/Game/BP/Squares/BP_Square_Block.BP_Square_Block_C") (Utilities|ClassIsChildOf (Utilities|GetClass (Variables|Move|IsThereSquare|GetHitActor_Move)) "/Game/BP/Squares/BP_Square_Block.BP_Square_Block_C"))))

(fn IsForward
  (return (Utilities|Enum|Equal(Enum) (Variables|Move|GetMoveDir) "NewEnumerator1")))

(fn IsShovel
  (return (Variables|/Game/BP/BP_GM.BP_GM_C|GetIsShovelActive (Variables|Ref|GetGameMode_Ref))))

(fn CallOffsetChunk|ChangeClog
  (params (Clog%20Coef :type Integer))
  (Default|CallOffsetChunk)
  (Status|Clog|ChangeClog Clog%20Coef))

(fn SetChunkRef
  (Utilities|IsValid (Variables|Ref|GetChunk_Ref)
    (:Is%20Not%20Valid
      (bind _returnvalue (Actor|GetActorOfClass "/Game/BP/BP_Chunk.BP_Chunk_C"))
      (Variables|Ref|SetChunk_Ref _returnvalue))))

(fn SetGreyLineRef
  (Utilities|IsValid (Variables|Ref|GetGreyLine_Ref)
    (:Is%20Not%20Valid
      (bind _returnvalue (Actor|GetActorOfClass "/Game/BP/BP_GreyLine.BP_GreyLine_C"))
      (Variables|Ref|SetGreyLine_Ref _returnvalue))))

(fn ClogtoLuck
  (Variables|Status|Clog|SetClogAmount_New (Variables|Status|Clog|GetChar_Clog))
  (Variables|Status|Clog|ClogtoLuck|SetClog%2819%29Counter (+ (Math|Integer|Absolute(Integer) (- (Variables|Status|Clog|GetClogAmount_Old) (Variables|Status|Clog|GetClogAmount_New))) (Variables|Status|Clog|ClogtoLuck|GetClog%2819%29Counter)))
  (if (>= (Variables|Status|Clog|GetChar_Clog) 90)
    (if (Math|Random|RandomBoolwithWeight 0.3)
      (Status|Luck|ChangeLuck -1)
      (if (>= (Variables|Status|Clog|ClogtoLuck|GetClog%2819%29Counter) 19) :!label _label
        (Variables|Status|Clog|ClogtoLuck|SetClog%2819%29Counter 0) ; reset counter
        (Status|Luck|ChangeLuck -1)
        (Default|CheckLuckChangeChancesMap (Variables|Ref|GetGameMode_Ref))))
    (else
      (goto _label))))

(fn SetCharStatusOldVariables
  (Utilities|Array|Clear (Variables|Status|Health|GetHealth_OverTurnArray))
  (Variables|Status|Health|SetHealth_OverTurn 0)
  (Variables|Status|Health|SetHealthAmount_Old (Variables|Status|Health|GetChar_Health))
  (Variables|Status|Clog|SetClogAmount_Old (Variables|Status|Clog|GetChar_Clog)))

(fn SpawnFlyingText
  (if (!= (Variables|Status|Health|GetHealth_OverTurn) 0)
    (Game|SpawnActorfromClass "/Game/BP/BP_FlyingStatusText.BP_FlyingStatusText_C" (Math|Transform|MakeTransform (Transformation|GetActorLocation) "0, 0, 0" "1.000000,1.000000,1.000000") "AdjustIfPossibleButAlwaysSpawn" 0 0)))

(fn DoChangeHealth
  (for _array_element (Variables|Status|Health|GetHealth_OverTurnArray)
    (Variables|Status|Health|SetHealth_OverTurn (+ _array_element (Variables|Status|Health|GetHealth_OverTurn))))
  (Variables|Status|Health|SetChar_Health (Math|Integer|Clamp(Integer) (+ (Variables|Status|Health|GetHealth_OverTurn) (Variables|Status|Health|GetChar_Health)) 0 100))
  (CallFunction|SpawnFlyingText)
  (return (<= (Variables|Status|Health|GetChar_Health) 0)))

(fn CreateGameOverWidget
  (params (is%20Health%200 :type Boolean))
  (if is%20Health%200
    (Default|SaveGameEvent (Variables|Ref|GetGameMode_Ref))
    (Variables|/Game/BP/BP_GM.BP_GM_C|SetIsMoveFinished (Variables|Ref|GetGameMode_Ref) false)
    (Variables|Move|SetMoveForward_CounterFlag false)
    (bind _foundwidgets (Widget|GetAllWidgetsOfClass "/Game/BP/UI/UI_InGame.UI_InGame_C" true))
    (for _array_element _foundwidgets
      (Utilities|IsValid _array_element
        (:Is%20Valid
          (Widget|RemovefromParent _array_element))))
    (bind _returnvalue (UserInterface|CreateWidget "/Game/BP/UI/UI_GameOver.UI_GameOver_C" (Variables|Ref|GetPlayerController_Ref)))
    (UserInterface|Viewport|AddtoViewport _returnvalue 0))
  (return))

(fn Destroyable)