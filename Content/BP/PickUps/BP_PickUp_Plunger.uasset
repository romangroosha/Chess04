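; Plunger pickup Blueprint, a child pickup that makes whoever collects it wear a plunger.
; BeginPlay runs the parent setup, then sets the weight AI uses when choosing this pickup.
; Before-destroy hooks for player and enemy characters each call WearPlunger on that character reference.
; Overlap and construction logic are left to the parent class.
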(event EventBeginPlay
  (|CallParentFunction)
  (Variables|Default|SetAIChoiceWeight 50))

(event Collision|EventActorBeginOverlap
  (params (OtherActor :type Actor%20Object%20Reference))
  (|CallParentFunction OtherActor) ; This node is disabled and will not be called.\nDrag off pins to build functionality.
)

(event EventTick
  (params (DeltaSeconds :type Float%20%28single-precision%29))
  (|CallParentFunction DeltaSeconds) ; This node is disabled and will not be called.\nDrag off pins to build functionality.
)

(event EventBeforeDestroyforEnemyChar
  (Default|WearPlunger (Variables|Default|GetEnemyCharacter_Ref)))

(event EventBeforeDestroyforCharacter
  (Default|WearPlunger (Variables|Default|GetCharacter_Ref)))

(fn ConstructionScript
  (|CallParentFunction))