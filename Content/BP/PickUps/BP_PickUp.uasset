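; BP_PickUp is a pickup actor that spins at a randomized yaw rate while a timeline animates its mesh height.
; On sphere overlap with the player character it calls an empty BeforeDestroy hook, apparently for child-specific effects, then destroys itself.
; Overlap with BP_GreyLine or any BP_PatrolEnemy subclass destroys it without that hook.
; It caches character and game mode references on BeginPlay, but the game mode pooling call is unwired.
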(event OnComponentBeginOverlap(SphereCollision)
  (params (OverlappedComponent :type Primitive%20Component%20Object%20Reference) (OtherActor :type Actor%20Object%20Reference) (OtherComp :type Primitive%20Component%20Object%20Reference) (OtherBodyIndex :type Integer) (bFromSweep :type Boolean) (SweepResult :type Hit%20Result%20Structure%20%28by%20ref%29))
  (if (== OtherActor (Variables|Ref|GetCharacter_Ref))
    (CallFunction|BeforeDestroyforCharacter)
    (Actor|DestroyActor :!label _label)
    (elif (== (Utilities|GetClass OtherActor) "/Game/BP/BP_GreyLine.BP_GreyLine_C")
      (goto _label)
      (elif (Utilities|ClassIsChildOf (Utilities|GetClass OtherActor) "/Game/BP/Enemies/BP_PatrolEnemy.BP_PatrolEnemy_C")
        (goto _label)))))

(event Custom|BeforeDestroy_ForCharacter)

(event EventBeginPlay
  (bind _pickupmesh (Variables|Default|GetPickUpMesh))
  (bind _relativelocation (Variables|/Script/Engine.SceneComponent|GetRelativeLocation _pickupmesh))
  (Ref|SetCharacterRef)
  (Ref|SetGameModeRef)
  (Variables|/Script/Engine.RotatingMovementComponent|SetRotationRate (Variables|Default|GetRotatingMovement) (Math|Rotator|MakeRotator 0.0 0.0 (Math|Conversions|ToFloat(Integer) (* (Math|Random|RandomIntegerinRange 1 3) 45))))
  (bind _location_z (Timeline|Timeline_0 PlayFromStart)
    (:Update
      (Transformation|SetRelativeLocation (Variables|Default|GetPickUpMesh) (Math|Vector|MakeVector (.x _relativelocation) (.y _relativelocation) _location_z) false false))))

(event Collision|EventActorBeginOverlap
  (params (OtherActor :type Actor%20Object%20Reference)))

(event EventTick
  (params (DeltaSeconds :type Float%20%28single-precision%29)))

(fn ConstructionScript)

(fn SetCharacterRef
  (Utilities|IsValid (Variables|Ref|GetCharacter_Ref)
    (:Is%20Not%20Valid
      (bind _returnvalue (Actor|GetActorOfClass "/Game/BP/BP_Character.BP_Character_C"))
      (Variables|Ref|SetCharacter_Ref _returnvalue))))

(fn SetGameModeRef
  (Utilities|IsValid (Variables|Ref|GetGameMode_Ref)
    (:Is%20Not%20Valid
      (bind _asbp_gm (Utilities|Casting|CastToBP_GM (Game|GetGameMode)))
      (Variables|Ref|SetGameMode_Ref _asbp_gm))))