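; BP_PickUp_Damage is a harmful pickup that lowers the health of the player or enemy character that takes it.
; On BeginPlay it sets the inherited HealDamage and AIChoiceWeight to negative values, reusing the heal variable for damage and weighting AI choice against it.
; The before-destroy events for each character type pass HealDamage to that character's WriteChangeHealth, leaving other pickup logic to the parent.
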(event EventBeginPlay
  (|CallParentFunction)
  (Variables|Default|SetHealDamage -4)
  (Variables|Default|SetAIChoiceWeight -15))

(event Collision|EventActorBeginOverlap
  (params (OtherActor :type Actor%20Object%20Reference))
  (|CallParentFunction OtherActor) ; This node is disabled and will not be called.\nDrag off pins to build functionality.
)

(event EventTick
  (params (DeltaSeconds :type Float%20%28single-precision%29))
  (|CallParentFunction DeltaSeconds) ; This node is disabled and will not be called.\nDrag off pins to build functionality.
)

(event EventBeforeDestroyforCharacter
  (Default|WriteChangeHealth (Variables|Default|GetCharacter_Ref) (Variables|Default|GetHealDamage)))

(event EventBeforeDestroyforEnemyChar
  (Default|WriteChangeHealth (Variables|Default|GetEnemyCharacter_Ref) (Variables|Default|GetHealDamage)))

(fn ConstructionScript
  (|CallParentFunction))