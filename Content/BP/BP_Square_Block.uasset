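; BP_Square_Block is a block square that turns into a regular square when destroyed.
; On BeginPlay it gives Cube1 a random yaw in 45-degree steps.
; The Destroyable event changes the character's clog, returns the block to the GameMode's square pool and pulls a BP_Square_Regular from it with the same parent and location.
; A separate pre-death function whitens and enlarges Cube0.
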(event EventBeginPlay
  (|CallParentFunction)
  (Transformation|SetRelativeRotation (Variables|Default|GetCube1) (Math|Rotator|MakeRotator 0.0 0.0 (Math|Conversions|ToFloat(Integer) (* (Math|Random|RandomIntegerinRange 0 8) 45))) false false))

(event Collision|EventActorBeginOverlap
  (params (OtherActor :type Actor%20Object%20Reference))
  (|CallParentFunction OtherActor) ; This node is disabled and will not be called.\nDrag off pins to build functionality.
)

(event EventTick
  (params (DeltaSeconds :type Float%20%28single-precision%29))
  ;[0.1146 0.1146 0.1146] Delta 0 to 1
  (if (>= (Variables|Default|GetDelta) 1.0)
    (Variables|Default|SetDelta 0.0)))

(event EventDestroyable
  (Destroyable|DestroySelfandSpawnNewSquare))

(fn ConstructionScript
  (|CallParentFunction))

(fn DestroySelfandSpawnNewSquare
  (LocalVariables|SetActor%20Location (.location (Transformation|GetActorTransform)))
  (LocalVariables|SetActor%20Transform (Transformation|GetActorTransform))
  (LocalVariables|SetActor%20Parent (Actor|GetAttachParentActor))
  (Default|ChangeClog (Variables|Default|GetCharacter_Ref) 10)
  (Default|AddtoSquarePool (Variables|Default|GetGameMode_Ref) self)
  (Default|GetfromSquarePool (Variables|Default|GetGameMode_Ref) "/Game/BP/BP_Square_Regular.BP_Square_Regular_C" (LocalVariables|GetActor%20Parent) (LocalVariables|GetActor%20Location)))

(fn CubeMeshPre-DeathTransform
  (Rendering|Material|SetMaterial (Variables|Default|GetCube_0) 0 "/Game/MATERIALS/MI_Square_White.MI_Square_White")
  (Transformation|SetRelativeTransform (Variables|Default|GetCube_0) (Math|Transform|MakeTransform "0, 0,100.000000" "0, 0, 0" "1.100000,1.100000,1.100000") false false))