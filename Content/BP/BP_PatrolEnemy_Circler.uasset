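; BP_PatrolEnemy_Circler is a patrol enemy that steps through a repeating four-leg movement pattern.
; Each MoveEvent call stores the current location, and a looping MultiGate picks the next leg in order.
; SetEnemyLocationNew adds that leg's offset from the 4Turns array to the current location.
; Timeline_EnemyMove then eases the actor between the stored and new locations with an EaseInOut curve.
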(event EventBeginPlay)

(event Collision|EventActorBeginOverlap
  (params (OtherActor :type Actor%20Object%20Reference)))

(event EventTick
  (params (DeltaSeconds :type Float%20%28single-precision%29)))

(event EventMoveEvent
  (params (Move :type Enum_Direction%20Enum :default "NewEnumerator0"))
  (Variables|move|SetEnemyLocation%20Old (.location (Transformation|GetActorTransform)))
  (Utilities|FlowControl|MultiGate false true -1
    (:Out%200
      (Utilities|SetEnemyLocationNew)
      (bind _0_to_1 (Timeline|Timeline_EnemyMove PlayFromStart)
        (:Update
          (Transformation|SetActorLocationAndRotation (Math|Interpolation|Ease "EaseInOut" _0_to_1 (Variables|move|GetEnemyLocation%20Old) (Variables|Move|GetEnemyLocation%20New) 3.0) "0, 0, 0"))))
    (:Out%201
      (Utilities|SetEnemyLocationNew 1)
      (Timeline|Timeline_EnemyMove PlayFromStart))
    (:Out%202
      (Utilities|SetEnemyLocationNew 2)
      (Timeline|Timeline_EnemyMove PlayFromStart))
    (:Out%203
      (Utilities|SetEnemyLocationNew 3)
      (Timeline|Timeline_EnemyMove PlayFromStart))))

(fn ConstructionScript
  (|CallParentFunction))