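; Player controller that turns directional input into movement events for the BP_Character in the level.
; On BeginPlay it finds and caches the character with GetActorOfClass, then sets it as the view target.
; The Left, Forward and Right input actions each pass a direction index to CallMoveEvent on press.
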(event EventBeginPlay
  (Ref|SetCharacterRef)
  (Game|Player|SetViewTargetwithBlend self (Variables|Ref|GetCharacter_Ref) 0.0 "VTBlend_Linear" 0.0 false))

(event Input|ActionEvents|InputActionForward
  (params (Key :type Key%20Structure :default "None"))
  (:Pressed
    (Default|CallMoveEvent 1)))

(event Input|ActionEvents|InputActionLeft
  (params (Key :type Key%20Structure :default "None"))
  (:Pressed
    (Default|CallMoveEvent)))

(event Input|ActionEvents|InputActionRight
  (params (Key :type Key%20Structure :default "None"))
  (:Pressed
    (Default|CallMoveEvent 2)))

(fn ConstructionScript)

(fn SetCharacterRef
  (Utilities|IsValid (Variables|Ref|GetCharacter_Ref)
    (:Is%20Not%20Valid
      (bind _returnvalue (Actor|GetActorOfClass "/Game/BP/BP_Character.BP_Character_C"))
      (Variables|Ref|SetCharacter_Ref _returnvalue))))