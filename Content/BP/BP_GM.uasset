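; Game mode that creates the main UI and manages object pools of squares and pickups for the game.
; On BeginPlay it pre-spawns 200 hidden, disabled actors per class key in the square and pickup chance maps.
; Get functions move a random pooled actor of a class into place, attach and activate it; add functions reset and hide returned actors.
; A separate function swaps both chance maps by the character's luck tier.
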(event EventBeginPlay
  (Ref|SetPlayerControllerRef)
  (Ref|SetChunkRef)
  (Ref|SetCharacterRef)
  (bind _returnvalue (UserInterface|CreateWidget "/Game/BP/UI/UI_Main.UI_Main_C" (Variables|Ref|GetPlayerController_Ref)))
  (UserInterface|Viewport|AddtoViewport _returnvalue 0)
  (ObjectPool|Create|CreateObjectPoolfromMap (Variables|ObjectPool|GetSquares_ObjectPool) (Variables|ChancesMaps|Default|GetSquareChancesMap))
  (ObjectPool|Create|CreateObjectPoolfromMap (Variables|ObjectPool|GetPickUps_ObjectPool) (Variables|ChancesMaps|Default|GetPickupsChancesMap)))

(event EventTick
  (params (DeltaSeconds :type Float%20%28single-precision%29)))

(fn ConstructionScript)

(fn SetPlayerControllerRef
  (Utilities|IsValid (Variables|Ref|GetPlayerController_Ref)
    (:Is%20Not%20Valid
      (bind _returnvalue (Actor|GetActorOfClass "/Game/BP/BP_PlayerController.BP_PlayerController_C"))
      (Variables|Ref|SetPlayerController_Ref _returnvalue))))

(fn CreateObjectPoolfromMap
  (params (Pool :type Array%20of%20Actor%20Object%20References) (Map :type Map%20of%20Actor%20Class%20References%20to%20Reals))
  (Utilities|Array|Clear Pool)
  (bind _keys (Utilities|Map|Keys Map))
  (bind _index (Utilities|FlowControl|ForLoopwithBreak 0 (Utilities|Array|LastIndex _keys))
    (:LoopBody
      (bind _index_2 (Utilities|FlowControl|ForLoopwithBreak 0 199)
        (:LoopBody
          (bind _keys_2 (Utilities|Map|Keys Map))
          (bind _returnvalue (Game|SpawnActorfromClass (Utilities|Array|Get(acopy) _keys_2 _index) (Math|Transform|MakeTransform (Math|Vector|MakeVector -1e+03 -1e+03 (Math|Conversions|ToFloat(Integer) _index_2)) "0, 0, 0" "0.000000,0.000000,0.000000") "AlwaysSpawn" 0 0))
          (Utilities|IsValid _returnvalue
            (:Is%20Valid
              (Utilities|Array|AddUnique Pool _returnvalue)
              (Rendering|SetActorHiddenInGame _returnvalue true)
              (Collision|SetActorEnableCollision _returnvalue false)
              (Actor|Tick|SetActorTickEnabled _returnvalue))))))
    (:Completed
      (return))))

(fn SetChunkRef
  (Utilities|IsValid (Variables|Ref|GetChunk_Ref)
    (:Is%20Not%20Valid
      (bind _returnvalue (Actor|GetActorOfClass "/Game/BP/BP_Chunk.BP_Chunk_C"))
      (Variables|Ref|SetChunk_Ref _returnvalue))))

(fn AddUniquetoObjectPool
  (params (Pool :type Array%20of%20Actor%20Object%20References) (Actor :type Actor%20Object%20Reference%20%28by%20ref%29))
  (LocalVariables|SetActor_Local Actor)
  (Class|InterfacePoolResetAble|PoolResetable(Message) (LocalVariables|GetActor_Local))
  (Rendering|SetActorHiddenInGame (LocalVariables|GetActor_Local) true)
  (Collision|SetActorEnableCollision (LocalVariables|GetActor_Local) false)
  (Actor|Tick|SetActorTickEnabled (LocalVariables|GetActor_Local))
  (bind _returnvalue (Utilities|Array|AddUnique Pool (LocalVariables|GetActor_Local)))
  (Transformation|SetActorTransform (LocalVariables|GetActor_Local) (Math|Transform|MakeTransform (Math|Vector|MakeVector -1e+03 -1e+03 (Math|Conversions|ToFloat(Integer) _returnvalue)) "0, 0, 0" "0.000000,0.000000,0.000000") false true))

(fn AddtoSquarePool
  (params (Actor :type Actor%20Object%20Reference%20%28by%20ref%29))
  (ObjectPool|Add|AddUniquetoObjectPool (Variables|ObjectPool|GetSquares_ObjectPool) Actor))

(fn AddtoPickupPool
  (params (Actor :type Actor%20Object%20Reference%20%28by%20ref%29))
  (ObjectPool|Add|AddUniquetoObjectPool (Variables|ObjectPool|GetPickUps_ObjectPool) Actor))

(fn GetfromObjectPool
  (params (Class :type Actor%20Class%20Reference) (Pool :type Array%20of%20Actor%20Object%20References) (Parent :type Actor%20Object%20Reference) (Location :type Vector))
  (LocalVariables|SetParent_Local Parent)
  (LocalVariables|SetLocation_Local Location)
  (bind _filteredarray (Utilities|Array|FilterArray Pool Class))
  (Utilities|IsValid (.OutItem (Utilities|Array|Random _filteredarray))
    (:Is%20Valid
      (bind _output_get (LocalVariables|SetRandomActor_Local (.OutItem (Utilities|Array|Random _filteredarray))))
      (Utilities|IsValid _output_get
        (:Is%20Valid
          (Transformation|SetActorTransform (LocalVariables|GetRandomActor_Local) (Math|Transform|MakeTransform (LocalVariables|GetLocation_Local) "0, 0, 0" "1.000000,1.000000,1.000000") false true)
          (Utilities|IsValid (LocalVariables|GetParent_Local)
            (:Is%20Valid
              (Utilities|IsValid (LocalVariables|GetRandomActor_Local)
                (:Is%20Valid
                  (Transformation|AttachActorToActor (LocalVariables|GetRandomActor_Local) (LocalVariables|GetParent_Local) "None" "KeepWorld" "KeepRelative" "KeepRelative" true)
                  (Utilities|IsValid (LocalVariables|GetRandomActor_Local)
                    (:Is%20Valid
                      (Rendering|SetActorHiddenInGame (LocalVariables|GetRandomActor_Local) false)
                      (Collision|SetActorEnableCollision (LocalVariables|GetRandomActor_Local) true)
                      (Utilities|IsValid (LocalVariables|GetRandomActor_Local)
                        (:Is%20Valid
                          (Actor|Tick|SetActorTickEnabled (LocalVariables|GetRandomActor_Local) true)
                          (Utilities|Array|RemoveItem Pool (LocalVariables|GetRandomActor_Local)))
                        (:Is%20Not%20Valid
                          (Development|PrintString "Random Actor is NOT valid (trying to Tick Enabled)" true true "(R=1.000000,G=0.193894,B=0.000000,A=1.000000)" 5.0))))
                    (:Is%20Not%20Valid
                      (Development|PrintString "Random Actor is NOT valid (trying to Hidden)" true true "(R=1.000000,G=0.193894,B=0.000000,A=1.000000)" 5.0))))
                (:Is%20Not%20Valid
                  (Development|PrintString "Random Actor is NOT valid (trying to Attach)" true true "(R=1.000000,G=0.193894,B=0.000000,A=1.000000)" 5.0))))
            (:Is%20Not%20Valid
              (Development|PrintString "Parent is NOT valid" true true "(R=1.000000,G=0.193894,B=0.000000,A=1.000000)" 5.0))))
        (:Is%20Not%20Valid
          (Development|PrintString "Random Actor is NOT valid (trying to Location)" true true "(R=1.000000,G=0.193894,B=0.000000,A=1.000000)" 5.0))))))

(fn GetfromSquarePool
  (params (Class :type Actor%20Class%20Reference) (Parent :type Actor%20Object%20Reference) (Location :type Vector))
  (ObjectPool|Get|GetfromObjectPool Class (Variables|ObjectPool|GetSquares_ObjectPool) Parent Location))

(fn GetfromPickupPool
  (params (Class :type Actor%20Class%20Reference) (Parent :type Actor%20Object%20Reference) (Location :type Vector))
  (ObjectPool|Get|GetfromObjectPool Class (Variables|ObjectPool|GetPickUps_ObjectPool) Parent Location))

(fn SetCharacterRef
  (Utilities|IsValid (Variables|Ref|GetCharacter_Ref)
    (:Is%20Not%20Valid
      (bind _returnvalue (Actor|GetActorOfClass "/Game/BP/BP_Character.BP_Character_C"))
      (Variables|Ref|SetCharacter_Ref _returnvalue))))

(fn CheckLuckChangeChancesMap
  (if (>= (Variables|/Game/BP/BP_Character.BP_Character_C|GetChar_Luck (Variables|Ref|GetCharacter_Ref)) 7)
    (Variables|ChancesMaps|Default|SetSquareChancesMap (Variables|ChancesMaps|Luck|7|GetSquareChancesMap_%287%29Luck))
    (Variables|ChancesMaps|Default|SetPickupsChancesMap (Variables|ChancesMaps|Luck|7|GetPickupsChancesMap_%287%29Luck))
    (if (>= (Variables|/Game/BP/BP_Character.BP_Character_C|GetChar_Luck (Variables|Ref|GetCharacter_Ref)) 9)
      (Variables|ChancesMaps|Default|SetSquareChancesMap (Variables|ChancesMaps|Luck|9|GetSquareChancesMap_%289%29Luck))
      (Variables|ChancesMaps|Default|SetPickupsChancesMap (Variables|ChancesMaps|Luck|9|GetPickupsChancesMap_%289%29Luck)))
    (elif (<= (Variables|/Game/BP/BP_Character.BP_Character_C|GetChar_Luck (Variables|Ref|GetCharacter_Ref)) 3)
      (Variables|ChancesMaps|Default|SetSquareChancesMap (Variables|ChancesMaps|Luck|3|GetSquareChancesMap_%283%29Luck))
      (Variables|ChancesMaps|Default|SetPickupsChancesMap (Variables|ChancesMaps|Luck|3|GetPickupsChancesMap_%283%29Luck))
      (if (<= (Variables|/Game/BP/BP_Character.BP_Character_C|GetChar_Luck (Variables|Ref|GetCharacter_Ref)) 1)
        (Variables|ChancesMaps|Default|SetSquareChancesMap (Variables|ChancesMaps|Luck|1|GetSquareChancesMap_%281%29Luck))
        (Variables|ChancesMaps|Default|SetPickupsChancesMap (Variables|ChancesMaps|Luck|1|GetPickupsChancesMap_%281%29Luck))))))