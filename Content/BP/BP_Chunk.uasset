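; BP_Chunk is a grid segment of an endlessly extending level, filled with squares and pickups.
; On BeginPlay it normalises weighted chance maps, sizes its triggers, then rolls each cell from BP_GM's object pools, skipping pickups on block squares.
; When the character crosses SpawnTrigger it spawns the next chunk in X; DestroyTrigger returns attached actors to the pools.
; The timeline movement and child-actor generation paths are unused.
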(event OnComponentBeginOverlap(SpawnTrigger)
  (params (OverlappedComponent :type Primitive%20Component%20Object%20Reference) (OtherActor :type Actor%20Object%20Reference) (OtherComp :type Primitive%20Component%20Object%20Reference) (OtherBodyIndex :type Integer) (bFromSweep :type Boolean) (SweepResult :type Hit%20Result%20Structure%20%28by%20ref%29))
  (if (== OtherActor (Variables|Ref|GetCharacter_Ref))
    (Utilities|FlowControl|DoOnce false
      (:Completed
        (Chunk|SpawnChunkatEnd)))))

(event OnComponentBeginOverlap(DestroyTrigger)
  (params (OverlappedComponent :type Primitive%20Component%20Object%20Reference) (OtherActor :type Actor%20Object%20Reference) (OtherComp :type Primitive%20Component%20Object%20Reference) (OtherBodyIndex :type Integer) (bFromSweep :type Boolean) (SweepResult :type Hit%20Result%20Structure%20%28by%20ref%29))
  (if (== OtherActor (Variables|Ref|GetCharacter_Ref))
    (Utilities|FlowControl|DoOnce false
      (:Completed
        (Chunk|ToObjPool "/Game/BP/BP_Square.BP_Square_C" (Variables|/Game/BP/BP_GM.BP_GM_C|GetSquares_ObjectPool (Variables|Ref|GetGameMode_Ref)))
        (Chunk|ToObjPool "/Game/BP/BP_PickUp.BP_PickUp_C" (Variables|/Game/BP/BP_GM.BP_GM_C|GetPickUps_ObjectPool (Variables|Ref|GetGameMode_Ref)))))))

(event Custom|Initialize
  (Ref|SetCharacterRef)
  (Ref|SetPlayerControllerRef)
  (Ref|SetGameModeRef)
  (EventDispatchers|AssignOffsetChunk (Variables|Ref|GetCharacter_Ref) (EventDispatchers|CreateEvent :!event Custom|OffsetChunk)))

(event Custom|OffsetChunk)

(event EventBeginPlay
  (CallFunction|Initialize)
  (Chances|SquarestoPercentage)
  (Chances|PickupstoPercentage)
  (Triggers|SizeandLocationOfTriggers)
  (Utilities|FlowControl|Delay 0.1)
  (bind _location (Utilities|LoopRows) ; Rows Y
    (:Loop%20Body
      (Chunk|GenerationUsingObjectPool _location) ; Generation
    )))

(fn ConstructionScript)

(fn SetCharacterRef
  (Utilities|IsValid (Variables|Ref|GetCharacter_Ref)
    (:Is%20Not%20Valid
      (bind _returnvalue (Actor|GetActorOfClass "/Game/BP/BP_Character.BP_Character_C"))
      (Variables|Ref|SetCharacter_Ref _returnvalue))))

(fn SetPlayerControllerRef
  (Utilities|IsValid (Variables|Ref|GetPlayerController_Ref)
    (:Is%20Not%20Valid
      (bind _returnvalue (Actor|GetActorOfClass "/Game/BP/BP_PlayerController.BP_PlayerController_C"))
      (Variables|Ref|SetPlayerController_Ref _returnvalue))))

(fn SetGameModeRef
  (Utilities|IsValid (Variables|Ref|GetGameMode_Ref)
    (:Is%20Not%20Valid
      (bind _asbp_gm (Utilities|Casting|CastToBP_GM (Game|GetGameMode)))
      (Variables|Ref|SetGameMode_Ref _asbp_gm))))

(fn SpawnChunkatEnd
  (bind _returnvalue (Transformation|GetActorLocation))
  (Game|SpawnActorfromClass "BP_Chunk_C" (Math|Transform|MakeTransform (Math|Vector|MakeVector (+ (* (Variables|Chunk|GetSizeOffset) (Variables|Chunk|GetAmount%20Columns%20X)) (.x _returnvalue)) (.y _returnvalue) (.z _returnvalue)) "0, 0, 0" "1.000000,1.000000,1.000000") "Undefined" 0 0))

(fn DoCentertheTrigger
  (return (Math|Conversions|ToFloat(Integer) (- (/ (* (Variables|Chunk|GetAmount%20Rows%20Y) (Variables|Chunk|GetSizeOffset)) 2) (/ (Variables|Chunk|GetSizeOffset) 2)))))

(fn WideOfTrigger
  (return (Math|Conversions|ToFloat(Integer) (/ (* (Variables|Chunk|GetAmount%20Rows%20Y) (Variables|Chunk|GetSizeOffset)) 2))))

(fn SizeandLocationOfTriggers
  (Transformation|SetRelativeLocation (Variables|Default|GetSpawnTrigger) (Math|Vector|MakeVector (Variables|Chunk|GetSpawTrig_LocX) (Triggers|DoCentertheTrigger) 0.0) false false)
  (Components|Box|SetBoxExtent (Variables|Default|GetSpawnTrigger) (Math|Vector|MakeVector 5.0 (Triggers|WideOfTrigger) 1.5e+02) true)
  (Transformation|SetRelativeLocation (Variables|Default|GetDestroyTrigger) (Math|Vector|MakeVector (Variables|Chunk|GetDestTrig_LocX) (Triggers|DoCentertheTrigger) 0.0) false false)
  (Components|Box|SetBoxExtent (Variables|Default|GetDestroyTrigger) (Math|Vector|MakeVector 5.0 (Triggers|WideOfTrigger) 1.5e+02) true))

(fn SetChunkLocationVariables
  (Variables|ChunkMove|SetChunk_Location_Old (Transformation|GetActorLocation))
  (Variables|ChunkMove|SetChunk_Location_New (+ "-100.000000,0.000000,0.000000" (Transformation|GetActorLocation))))

(fn GenerationUsingAddChildActorComp
  (params (Vector :type Vector))
  (LocalVariables|SetRelativeLocation Vector)
  (bind _index (Chances|ChancesCompute (Variables|Chances|Square|GetSquare_Keys) (Variables|Chances|Square|GetSquare_Values))) ; Squares
  (bind _returnvalue (AddComponent|AddChildActorComponent false (Math|Transform|MakeTransform (LocalVariables|GetRelativeLocation) "0, 0, 0" "1.000000,1.000000,1.000000"))) ; Spawn Square
  (ChildActorComponent|SetChildActorClass _returnvalue (Utilities|Array|Get(acopy) (Variables|Chances|Square|GetSquare_Keys) _index))
  (if (!= (Utilities|Array|Get(acopy) (Variables|Chances|Square|GetSquare_Keys) _index) "/Game/BP/BP_Square_Block.BP_Square_Block_C")
    (bind _index_2 (Chances|ChancesCompute (Variables|Chances|PickUps|GetPickups_Keys) (Variables|Chances|PickUps|GetPickups_Values))) ; PickUps
    (bind _returnvalue_2 (AddComponent|AddChildActorComponent false (Math|Transform|MakeTransform (LocalVariables|GetRelativeLocation) "0, 0, 0" "1.000000,1.000000,1.000000"))) ; Spawn PickUps
    (ChildActorComponent|SetChildActorClass _returnvalue_2 (Utilities|Array|Get(acopy) (Variables|Chances|PickUps|GetPickups_Keys) _index_2))))

(fn SquarestoPercentage
  (Utilities|FlowControl|Sequence
    (:then_0
      (bind _keys (Utilities|Map|Keys (Variables|Chances|Square|GetSquareChancesMap)))
      (Variables|Chances|Square|SetSquare_Keys _keys)
      (bind _values (Utilities|Map|Values (Variables|Chances|Square|GetSquareChancesMap)))
      (Variables|Chances|Square|SetSquare_Values _values))
    (:then_1
      (for _array_element (Variables|Chances|Square|GetSquare_Values)
        (LocalVariables|SetSumm (+ _array_element (LocalVariables|GetSumm)))))
    (:then_2
      (for _array_element_2 (Variables|Chances|Square|GetSquare_Values)
        (Utilities|Array|Add (LocalVariables|GetValues_Local) (/ (* _array_element_2 1e+02) (LocalVariables|GetSumm)))))
    (:then_3
      (Utilities|Array|Clear (Variables|Chances|Square|GetSquare_Values))
      (Variables|Chances|Square|SetSquare_Values (LocalVariables|GetValues_Local)))))

(fn PickupstoPercentage
  (Utilities|FlowControl|Sequence
    (:then_0
      (bind _keys (Utilities|Map|Keys (Variables|Chances|PickUps|GetPickupsChancesMap)))
      (Variables|Chances|PickUps|SetPickups_Keys _keys)
      (bind _values (Utilities|Map|Values (Variables|Chances|PickUps|GetPickupsChancesMap)))
      (Variables|Chances|PickUps|SetPickups_Values _values))
    (:then_1
      (for _array_element (Variables|Chances|PickUps|GetPickups_Values)
        (LocalVariables|SetSumm (+ _array_element (LocalVariables|GetSumm)))))
    (:then_2
      (for _array_element_2 (Variables|Chances|PickUps|GetPickups_Values)
        (Utilities|Array|Add (LocalVariables|GetValues_Local) (/ (* _array_element_2 1e+02) (LocalVariables|GetSumm)))))
    (:then_3
      (Utilities|Array|Clear (Variables|Chances|PickUps|GetPickups_Values))
      (Variables|Chances|PickUps|SetPickups_Values (LocalVariables|GetValues_Local)))))

(fn ChancesCompute
  (params (Keys :type Array%20of%20Actor%20Class%20References) (Values :type Array%20of%20Floats%20%28double-precision%29))
  (LocalVariables|SetRandomFloat (Math|Random|RandomFloatinRange 1.0 1e+02))
  (bind _index (Utilities|FlowControl|ForLoopwithBreak 0 (Utilities|Array|LastIndex Keys) :!label _label)
    (:LoopBody
      (bind _output_get (LocalVariables|SetLoopIndex _index))
      (LocalVariables|SetInRange? (Math|Float|InRange(Float) (LocalVariables|GetRandomFloat) (LocalVariables|GetSumm) (+ (Utilities|Array|Get(acopy) Values _output_get) (LocalVariables|GetSumm)) false))
      (LocalVariables|SetSumm (+ (Utilities|Array|Get(acopy) Values _output_get) (LocalVariables|GetSumm)))
      (if (LocalVariables|GetInRange?)
        (goto _label Break)))
    (:Completed
      (return (LocalVariables|GetLoopIndex) (Utilities|Array|Get(acopy) Keys (LocalVariables|GetLoopIndex))))))

(fn GenerationUsingObjectPool
  (params (Relative :type Vector))
  (LocalVariables|SetLocation (+ Relative (Transformation|GetActorLocation)))
  (bind _class (Chances|ChancesCompute (Variables|Chances|Square|GetSquare_Keys) (Variables|Chances|Square|GetSquare_Values))) ; Squares
  (Default|GetfromSquarePool (Variables|Ref|GetGameMode_Ref) _class self (LocalVariables|GetLocation))
  (if (!= _class "/Game/BP/BP_Square_Block.BP_Square_Block_C") ; Get Not Block
    (bind _class_2 (Chances|ChancesCompute (Variables|Chances|PickUps|GetPickups_Keys) (Variables|Chances|PickUps|GetPickups_Values))) ; PickUps
    (Default|GetfromPickupPool (Variables|Ref|GetGameMode_Ref) _class_2 self (LocalVariables|GetLocation))))

(fn FromObjPooltoSpawn
  (params (Pool :type Array%20of%20Actor%20Object%20References) (Keys :type Array%20of%20Actor%20Class%20References) (RelativeLocation :type Vector) (Class%20Index :type Integer)))

(fn ToObjPool
  (params (ParentClass :type Object%20Class%20Reference) (Pool :type Array%20of%20Actor%20Object%20References))
  (for _array_element (Actor|GetAttachedActors true false)
    (bind _output_get (LocalVariables|SetAttachedActor_Local _array_element))
    (Utilities|IsValid _output_get
      (:Is%20Valid
        (if (Utilities|ClassIsChildOf (Utilities|GetClass _output_get) ParentClass)
          (Default|AddUniquetoObjectPool (Variables|Ref|GetGameMode_Ref) Pool (LocalVariables|GetAttachedActor_Local)))))))