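; BP_OldStartChunk is a starting level chunk that builds a grid of randomly picked Regular, Damage, Luck or Block tiles as child actors on BeginPlay.
; It binds to the player controller's move event and, for index -1, eases itself backward along X with a timeline, ignoring input until finished.
; Two sized box triggers respond to the character, one spawning the next BP_Chunk at the grid's far end, the other destroying this chunk.
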(event OnComponentBeginOverlap(DestroyTrigger)
  (params (OverlappedComponent :type Primitive%20Component%20Object%20Reference) (OtherActor :type Actor%20Object%20Reference) (OtherComp :type Primitive%20Component%20Object%20Reference) (OtherBodyIndex :type Integer) (bFromSweep :type Boolean) (SweepResult :type Hit%20Result%20Structure%20%28by%20ref%29))
  (if (== OtherActor (Variables|Ref|GetCharacter_Ref))
    (Utilities|FlowControl|DoOnce false
      (:Completed
        (Actor|DestroyActor)))
    (else
      (Utilities|FlowControl|DoOnce false))))

(event OnComponentBeginOverlap(SpawnTrigger)
  (params (OverlappedComponent :type Primitive%20Component%20Object%20Reference) (OtherActor :type Actor%20Object%20Reference) (OtherComp :type Primitive%20Component%20Object%20Reference) (OtherBodyIndex :type Integer) (bFromSweep :type Boolean) (SweepResult :type Hit%20Result%20Structure%20%28by%20ref%29))
  (bind _returnvalue (Transformation|GetActorLocation))
  (if (== OtherActor (Variables|Ref|GetCharacter_Ref))
    (Utilities|FlowControl|DoOnce false
      (:Completed
        (Game|SpawnActorfromClass "/Game/BP/BP_Chunk.BP_Chunk_C" (Math|Transform|MakeTransform (Math|Vector|MakeVector (+ (* (Variables|MakeChunk|GetSizeOffset) (Variables|MakeChunk|GetAmount%20Columns%20X)) (.x _returnvalue)) (.y _returnvalue) (.z _returnvalue)) "0, 0, 0" "1.000000,1.000000,1.000000") "Undefined" 0 0)))
    (else
      (Utilities|FlowControl|DoOnce false))))

(event Custom|MoveEvent
  (params (Index :type Integer))
  (if (== Index -1)
    (if (Variables|MoveChunk|GetIsMoveFinished)
      (Variables|MoveChunk|SetIsMoveFinished false)
      (Variables|MoveChunk|SetChunk_Location_Old (Transformation|GetActorLocation))
      (Variables|MoveChunk|SetChunk_Location_New (+ "-100.000000,0,0" (Transformation|GetActorLocation)))
      (bind _0_to_1 (Timeline|Timeline_0 PlayFromStart)
        (:Update
          (Variables|MoveChunk|SetIsMoveFinished false)
          (Transformation|SetActorLocation (Math|Interpolation|Ease "EaseInOut" _0_to_1 (Variables|MoveChunk|GetChunk_Location_Old) (Variables|MoveChunk|GetChunk_Location_New) 3.0) false false))
        (:Finished
          (Variables|MoveChunk|SetIsMoveFinished true))))))

(event EventBeginPlay
  (bind _returnvalue (Transformation|GetActorLocation))
  (Ref|SetCharacterRef)
  (Ref|SetPlayerControllerRef)
  (EventDispatchers|AssignMoveEvent (Variables|Ref|GetPlayerController_Ref) (EventDispatchers|CreateEvent :!event Custom|MoveEvent))
  (Transformation|SetActorLocation (Math|Vector|MakeVector (+ (/ (Variables|MakeChunk|GetSizeOffset) 2) (.x _returnvalue)) (+ (/ (Variables|MakeChunk|GetSizeOffset) 2) (.y _returnvalue)) 0.0) false false)
  (for _index (range 0 (- (Variables|MakeChunk|GetAmount%20Columns%20X) 1))
    (for _index_2 (range 0 (- (Variables|MakeChunk|GetAmount%20Rows%20Y) 1))
      (switch int (Math|Random|RandomIntegerinRange 0 3)
        (:0
          (AddComponent|AddChildActorComponent false (Math|Transform|MakeTransform (Math|Vector|MakeVector (Math|Conversions|ToFloat(Integer) (* _index (Variables|MakeChunk|GetSizeOffset))) (Math|Conversions|ToFloat(Integer) (* _index_2 (Variables|MakeChunk|GetSizeOffset))) 0.0) "0, 0, 0" "1.000000,1.000000,1.000000")) ; Regular
        )
        (:1
          (AddComponent|AddChildActorComponent false (Math|Transform|MakeTransform (Math|Vector|MakeVector (Math|Conversions|ToFloat(Integer) (* _index (Variables|MakeChunk|GetSizeOffset))) (Math|Conversions|ToFloat(Integer) (* _index_2 (Variables|MakeChunk|GetSizeOffset))) 0.0) "0, 0, 0" "1.000000,1.000000,1.000000")) ; Damage
        )
        (:2
          (AddComponent|AddChildActorComponent false (Math|Transform|MakeTransform (Math|Vector|MakeVector (Math|Conversions|ToFloat(Integer) (* _index (Variables|MakeChunk|GetSizeOffset))) (Math|Conversions|ToFloat(Integer) (* _index_2 (Variables|MakeChunk|GetSizeOffset))) 0.0) "0, 0, 0" "1.000000,1.000000,1.000000")) ; Luck
        )
        (:3
          (AddComponent|AddChildActorComponent false (Math|Transform|MakeTransform (Math|Vector|MakeVector (Math|Conversions|ToFloat(Integer) (* _index (Variables|MakeChunk|GetSizeOffset))) (Math|Conversions|ToFloat(Integer) (* _index_2 (Variables|MakeChunk|GetSizeOffset))) 0.0) "0, 0, 0" "1.000000,1.000000,1.000000")) ; Block
        ))))
  (Transformation|SetRelativeLocation (Variables|Default|GetSpawnTrigger) (Math|Vector|MakeVector 1e+02 (Math|Conversions|ToFloat(Integer) (- (/ (* (Variables|MakeChunk|GetAmount%20Rows%20Y) (Variables|MakeChunk|GetSizeOffset)) 2) (/ (Variables|MakeChunk|GetSizeOffset) 2))) 0.0) false false)
  (Components|Box|SetBoxExtent (Variables|Default|GetSpawnTrigger) (Math|Vector|MakeVector 5.0 (Math|Conversions|ToFloat(Integer) (/ (* (Variables|MakeChunk|GetAmount%20Rows%20Y) (Variables|MakeChunk|GetSizeOffset)) 2)) 1.5e+02) true)
  (Transformation|SetRelativeLocation (Variables|Default|GetDestroyTrigger) (Math|Vector|MakeVector 1.2e+03 (Math|Conversions|ToFloat(Integer) (- (/ (* (Variables|MakeChunk|GetAmount%20Rows%20Y) (Variables|MakeChunk|GetSizeOffset)) 2) (/ (Variables|MakeChunk|GetSizeOffset) 2))) 0.0) false false)
  (Components|Box|SetBoxExtent (Variables|Default|GetDestroyTrigger) (Math|Vector|MakeVector 5.0 (Math|Conversions|ToFloat(Integer) (* (* (Variables|MakeChunk|GetAmount%20Rows%20Y) (Variables|MakeChunk|GetSizeOffset)) 1)) 1.5e+02) true))

(fn ConstructionScript)

(fn SetCharacterRef
  (Utilities|IsValid (Variables|Ref|GetCharacter_Ref)
    (:Is%20Not%20Valid
      (bind _returnvalue (Actor|GetActorOfClass "/Game/BP/BP_Character.BP_Character_C"))
      (Variables|Ref|SetCharacter_Ref _returnvalue))))

(fn SetPlayerControllerRef
  (Utilities|IsValid (Variables|Ref|GetPlayerController_Ref)
    (:Is%20Not%20Valid
      (bind _returnvalue (Actor|GetActorOfClass "/Game/BP/BP_PlayerController.BP_PlayerController_C"))
      (Variables|Ref|SetPlayerController_Ref _returnvalue))))