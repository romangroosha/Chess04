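; BP_FirstLine is an actor with a collision box that spans the first line of the BP_Chunk grid.
; On BeginPlay it finds the chunk actor by class, waits briefly, then sizes and shifts the box using the chunk's SizeOffset and Y row count.
; The box forms a thin strip along X covering all rows along Y.
; Its overlap event is bound but has no logic.
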(event OnComponentBeginOverlap(FirstLineCollision)
  (params (OverlappedComponent :type Primitive%20Component%20Object%20Reference) (OtherActor :type Actor%20Object%20Reference) (OtherComp :type Primitive%20Component%20Object%20Reference) (OtherBodyIndex :type Integer) (bFromSweep :type Boolean) (SweepResult :type Hit%20Result%20Structure%20%28by%20ref%29)))

(event EventBeginPlay
  (bind _firstlinecollision (Variables|Default|GetFirstLineCollision))
  (bind _chunk_ref (Variables|Ref|GetChunk_Ref))
  (bind _chunk_ref_2 (Variables|Ref|GetChunk_Ref))
  (bind _returnvalue (Transformation|GetWorldLocation _firstlinecollision))
  (Ref|SetChunkRef)
  (Utilities|FlowControl|Delay 0.1)
  (Components|Box|SetBoxExtent (Variables|Default|GetFirstLineCollision) (Math|Vector|MakeVector (Math|Conversions|ToFloat(Integer) (/ (Variables|/Game/BP/BP_Chunk.BP_Chunk_C|GetSizeOffset (Variables|Ref|GetChunk_Ref)) 4)) (/ (* (Variables|/Game/BP/BP_Chunk.BP_Chunk_C|GetSizeOffset _chunk_ref) (Variables|/Game/BP/BP_Chunk.BP_Chunk_C|GetAmount%20Rows%20Y _chunk_ref)) 2) 5e+01) true)
  (Transformation|SetWorldLocation (Variables|Default|GetFirstLineCollision) (Math|Vector|MakeVector (+ (/ (Variables|/Game/BP/BP_Chunk.BP_Chunk_C|GetSizeOffset (Variables|Ref|GetChunk_Ref)) 4) (.x _returnvalue)) (+ (.y _returnvalue) (/ (* (Variables|/Game/BP/BP_Chunk.BP_Chunk_C|GetSizeOffset _chunk_ref_2) (Variables|/Game/BP/BP_Chunk.BP_Chunk_C|GetAmount%20Rows%20Y _chunk_ref_2)) 2)) 0.0) false false))

(fn ConstructionScript)

(fn SetChunkRef
  (Utilities|IsValid (Variables|Ref|GetChunk_Ref)
    (:Is%20Not%20Valid
      (bind _returnvalue (Actor|GetActorOfClass "/Game/BP/BP_Chunk.BP_Chunk_C"))
      (Variables|Ref|SetChunk_Ref _returnvalue))))