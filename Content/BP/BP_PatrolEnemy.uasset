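; BP_PatrolEnemy is an early patrol enemy Blueprint, so far containing only setup for reacting to the player controller's moves.
; On BeginPlay it finds and caches BP_Character and BP_PlayerController through GetActorOfClass, guarded by validity checks.
; It then assigns an event to the controller's MoveEvent dispatcher.
; The MoveEvent handler, overlap and Tick are empty, so no patrol behavior exists yet, and the character reference goes unused.
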(event Custom|MoveEvent
  (params (Move :type Enum_Direction%20Enum :default "NewEnumerator0")))

(event EventBeginPlay
  (ref|SetCharacterRef)
  (Ref|SetPlayerControllerRef)
  (EventDispatchers|AssignMoveEvent (Variables|Ref|GetPlayerController_Ref) (EventDispatchers|CreateEvent :!event Custom|MoveEvent)))

(event Collision|EventActorBeginOverlap
  (params (OtherActor :type Actor%20Object%20Reference)))

(event EventTick
  (params (DeltaSeconds :type Float%20%28single-precision%29)))

(fn ConstructionScript)

(fn SetCharacterRef
  (Utilities|IsValid (Variables|ref|GetCharacter_Ref)
    (:Is%20Not%20Valid
      (bind _returnvalue (Actor|GetActorOfClass "/Game/BP/BP_Character.BP_Character_C"))
      (Variables|ref|SetCharacter_Ref _returnvalue))))

(fn SetPlayerControllerRef
  (Utilities|IsValid (Variables|Ref|GetPlayerController_Ref)
    (:Is%20Not%20Valid
      (bind _returnvalue (Actor|GetActorOfClass "/Game/BP/BP_PlayerController.BP_PlayerController_C"))
      (Variables|Ref|SetPlayerController_Ref _returnvalue))))