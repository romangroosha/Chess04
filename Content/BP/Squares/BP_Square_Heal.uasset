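; Board square that heals whichever character lands on it, player or enemy.
; BeginPlay sets the heal amount and an AI choice weight after running the parent's setup.
; The CharacterOverlap and EnemyCharOverlap events pass that amount to the matching character reference's WriteChangeHealth.
; The local box overlap event is empty, and an IsCharacter helper checks for an exact BP_Character class.
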(event OnComponentBeginOverlap(BoxTrigger)
  (params (OverlappedComponent :type Primitive%20Component%20Object%20Reference) (OtherActor :type Actor%20Object%20Reference) (OtherComp :type Primitive%20Component%20Object%20Reference) (OtherBodyIndex :type Integer) (bFromSweep :type Boolean) (SweepResult :type Hit%20Result%20Structure%20%28by%20ref%29)))

(event EventBeginPlay
  (|CallParentFunction)
  (Variables|Default|SetDamageHeal 5)
  (Variables|Default|SetAIChoiceWeight 20))

(event Collision|EventActorBeginOverlap
  (params (OtherActor :type Actor%20Object%20Reference))
  (|CallParentFunction OtherActor) ; This node is disabled and will not be called.\nDrag off pins to build functionality.
)

(event EventTick
  (params (DeltaSeconds :type Float%20%28single-precision%29))
  (|CallParentFunction DeltaSeconds) ; This node is disabled and will not be called.\nDrag off pins to build functionality.
)

(event EventCharacterOverlap
  (Default|WriteChangeHealth (Variables|Default|GetCharacter_Ref) (Variables|Default|GetDamageHeal)))

(event EventEnemyCharOverlap
  (Default|WriteChangeHealth (Variables|Default|GetEnemyCharacter_Ref) (Variables|Default|GetDamageHeal)))

(fn ConstructionScript
  (|CallParentFunction))