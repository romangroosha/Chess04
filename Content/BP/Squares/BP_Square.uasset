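; BP_Square is a level square that shows player and enemy highlights and turns white when a BP_GreyLine overlaps it.
; Light events show each highlight a tick later; the controller's move event clears the player's, while certain character move states clear the enemy's.
; Grey-line overlap also drops the trigger and disables its overlaps.
; PoolResetAble restores material, trigger location and overlap setting saved at BeginPlay, so pooled squares can be reused.
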(event OnComponentBeginOverlap(BoxTrigger)
  (params (OverlappedComponent :type Primitive%20Component%20Object%20Reference) (OtherActor :type Actor%20Object%20Reference) (OtherComp :type Primitive%20Component%20Object%20Reference) (OtherBodyIndex :type Integer) (bFromSweep :type Boolean) (SweepResult :type Hit%20Result%20Structure%20%28by%20ref%29))
  (if (== (Utilities|GetClass OtherActor) "/Game/BP/BP_GreyLine.BP_GreyLine_C")
    (Rendering|Material|SetMaterial (Variables|Default|GetColor%20Plane) 0 "/Game/MATERIALS/MI_Square_White.MI_Square_White")
    (Transformation|SetRelativeLocation (Variables|Default|GetBoxTrigger) "0, 0,-200.000000" false true)
    (Variables|/Script/Engine.PrimitiveComponent|SetbGenerateOverlapEvents (Variables|Default|GetBoxTrigger) false)))

(event Custom|RememberForReset
  (Variables|Remember|SetRememberMaterial (Rendering|Material|GetMaterial (Variables|Default|GetColor%20Plane) 0))
  (Variables|Remember|SetRememberLocation (Variables|/Script/Engine.SceneComponent|GetRelativeLocation (Variables|Default|GetBoxTrigger)))
  (Variables|Remember|SetRememberGenerateOverlap (Variables|/Script/Engine.PrimitiveComponent|GetbGenerateOverlapEvents (Variables|Default|GetBoxTrigger))))

(event Custom|Move_Event
  (params (Move :type Enum_Direction%20Enum :default "NewEnumerator0"))
  (Rendering|SetVisibility (Variables|Default|GetLighted%20Plane) false false))

(event Custom|EnemyMove_Event
  (params (CharState :type Enum_CharacterStates%20Enum :default "NewEnumerator7"))
  (switch Utilities|FlowControl|Switch|SwitchonEnum_CharacterStates CharState
    (:NewEnumerator2
      _)
    (:NewEnumerator3
      _)
    (:NewEnumerator6
      _))
  (Rendering|SetVisibility (Variables|Default|GetEnemyLighted%20Plane) false false)
  (Ref|SetCharacterRef))

(event EventBeginPlay
  (Ref|SetChunkRef)
  (Ref|SetPlayerControllerRef)
  (Ref|SetCharacterRef)
  (Ref|SetGameModeRef)
  (EventDispatchers|AssignMoveEvent (Variables|Ref|GetPlayerController_Ref) (EventDispatchers|CreateEvent :!event Custom|Move_Event))
  (CallFunction|RememberforReset)
  (Utilities|IsCharacterRefValid)
  (EventDispatchers|AssignEnemyMove (Variables|Ref|GetCharacter_Ref) (EventDispatchers|CreateEvent :!event Custom|EnemyMove_Event)))

(event Collision|EventActorBeginOverlap
  (params (OtherActor :type Actor%20Object%20Reference)))

(event EventTick
  (params (DeltaSeconds :type Float%20%28single-precision%29)))

(event EventLightSquare
  (Utilities|FlowControl|DelayUntilNextTick)
  (Rendering|SetVisibility (Variables|Default|GetLighted%20Plane) true false))

(event EventPoolResetAble
  (Rendering|Material|SetMaterial (Variables|Default|GetColor%20Plane) 0 (Variables|Remember|GetRememberMaterial))
  (Transformation|SetRelativeLocation (Variables|Default|GetBoxTrigger) (Variables|Remember|GetRememberLocation) false true)
  (Variables|/Script/Engine.PrimitiveComponent|SetbGenerateOverlapEvents (Variables|Default|GetBoxTrigger) (Variables|Remember|GetRememberGenerateOverlap)))

(event EventEnemyLightSquare
  (Utilities|FlowControl|DelayUntilNextTick)
  (Rendering|SetVisibility (Variables|Default|GetEnemyLighted%20Plane) true false))

(fn ConstructionScript)

(fn SetPlayerControllerRef
  (Utilities|IsValid (Variables|Ref|GetPlayerController_Ref)
    (:Is%20Not%20Valid
      (bind _returnvalue (Actor|GetActorOfClass "/Game/BP/BP_PlayerController.BP_PlayerController_C"))
      (Variables|Ref|SetPlayerController_Ref _returnvalue))))

(fn SetCharacterRef
  (Utilities|IsValid (Variables|Ref|GetCharacter_Ref)
    (:Is%20Not%20Valid
      (bind _returnvalue (Actor|GetActorOfClass "/Game/BP/BP_Character.BP_Character_C"))
      (Variables|Ref|SetCharacter_Ref _returnvalue))))

(fn SetChunkRef
  (Utilities|IsValid (Variables|Ref|GetChunk_Ref)
    (:Is%20Not%20Valid
      (bind _returnvalue (Actor|GetActorOfClass "/Game/BP/BP_Chunk.BP_Chunk_C"))
      (Variables|Ref|SetChunk_Ref _returnvalue))))

(fn SetGameModeRef
  (Utilities|IsValid (Variables|Ref|GetGameMode_Ref)
    (:Is%20Not%20Valid
      (bind _asbp_gm (Utilities|Casting|CastToBP_GM (Game|GetGameMode)))
      (Variables|Ref|SetGameMode_Ref _asbp_gm))))