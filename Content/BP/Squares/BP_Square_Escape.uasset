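; BP_Square_Escape is a board square labeled "ESCAPE" that ends the game when the player or enemy character reaches it.
; On BeginPlay it sets its label text and gives itself an AI choice weight of 100.
; Overlap events from its parent square flag the player or enemy as escaped on the GameMode and open that character's game-over widget.
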(event OnComponentBeginOverlap(BoxTrigger)
  (params (OverlappedComponent :type Primitive%20Component%20Object%20Reference) (OtherActor :type Actor%20Object%20Reference) (OtherComp :type Primitive%20Component%20Object%20Reference) (OtherBodyIndex :type Integer) (bFromSweep :type Boolean) (SweepResult :type Hit%20Result%20Structure%20%28by%20ref%29)))

(event EventBeginPlay
  (|CallParentFunction)
  (CallFunction|TextSettings (Variables|Default|GetColor) "ESCAPE" 24.0)
  (Variables|Default|SetAIChoiceWeight 100))

(event Collision|EventActorBeginOverlap
  (params (OtherActor :type Actor%20Object%20Reference))
  (|CallParentFunction OtherActor) ; This node is disabled and will not be called.\nDrag off pins to build functionality.
)

(event EventTick
  (params (DeltaSeconds :type Float%20%28single-precision%29))
  (|CallParentFunction DeltaSeconds) ; This node is disabled and will not be called.\nDrag off pins to build functionality.
)

(event EventCharacterOverlap
  (Variables|/Game/BP/BP_GM.BP_GM_C|SetIsEscaped (Variables|Default|GetGameMode_Ref) true)
  (Default|CreateGameOverWidget (Variables|Default|GetCharacter_Ref) true))

(event EventEnemyCharOverlap
  (Variables|/Game/BP/BP_GM.BP_GM_C|SetIsEnemyEscaped (Variables|Default|GetGameMode_Ref) true)
  (Default|CreateGameOverWidget (Variables|Default|GetEnemyCharacter_Ref) true))

(fn ConstructionScript
  (|CallParentFunction))