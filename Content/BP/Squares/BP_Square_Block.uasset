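; Blueprint for a block square, a square variant that can be destroyed and replaced by a regular square.
; On BeginPlay it gives Cube1 a random yaw in 45-degree steps.
; The Destroyable event adds clog to the character, spawns BP_Square_Regular in place under the same parent, then destroys itself, leaving square-pool calls unused.
; A pre-death function whitens, repositions and slightly enlarges Cube0.
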(event EventBeginPlay
  (|CallParentFunction)
  (Transformation|SetRelativeRotation (Variables|Default|GetCube1) (Math|Rotator|MakeRotator 0.0 0.0 (Math|Conversions|ToFloat(Integer) (* (Math|Random|RandomIntegerinRange 0 8) 45))) false false))

(event Collision|EventActorBeginOverlap
  (params (OtherActor :type Actor%20Object%20Reference))
  (|CallParentFunction OtherActor) ; This node is disabled and will not be called.\nDrag off pins to build functionality.
)

(event EventDestroyable
  (Destroyable|DestroySelfandSpawnNewSquare))

(fn ConstructionScript
  (|CallParentFunction))

(fn DestroySelfandSpawnNewSquare
  (LocalVariables|SetActor%20Location (.location (Transformation|GetActorTransform)))
  (LocalVariables|SetActor%20Parent (Actor|GetAttachParentActor))
  (Default|ChangeClog (Variables|Default|GetCharacter_Ref) 10)
  (bind _returnvalue (Game|SpawnActorfromClass "/Game/BP/Squares/BP_Square_Regular.BP_Square_Regular_C" (Math|Transform|MakeTransform (LocalVariables|GetActor%20Location) "0, 0, 0" "1.000000,1.000000,1.000000") "Undefined" 0 0))
  (Transformation|AttachActorToActor _returnvalue (LocalVariables|GetActor%20Parent) "None" "KeepWorld" "KeepRelative" "KeepRelative" true)
  (Actor|DestroyActor))

(fn CubeMeshPre-DeathTransform
  (Rendering|Material|SetMaterial (Variables|Default|GetCube_0) 0 "/Game/MATERIALS/MI_Square_White.MI_Square_White")
  (Transformation|SetRelativeTransform (Variables|Default|GetCube_0) (Math|Transform|MakeTransform "0, 0,100.000000" "0, 0, 0" "1.100000,1.100000,1.100000") false false))