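; BP_Square is a poolable square tile that can light up and turns white when a BP_FirstLine actor overlaps its trigger.
; LightSquare shows the lit plane a tick later, and Move_Event, apparently bound through the player controller, hides it.
; The overlap also disables the trigger by hiding and sinking it.
; PoolResetAble restores the material and trigger state cached at BeginPlay; a timeline color fade is left unwired.
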(event OnComponentBeginOverlap(BoxTrigger)
  (params (OverlappedComponent :type Primitive%20Component%20Object%20Reference) (OtherActor :type Actor%20Object%20Reference) (OtherComp :type Primitive%20Component%20Object%20Reference) (OtherBodyIndex :type Integer) (bFromSweep :type Boolean) (SweepResult :type Hit%20Result%20Structure%20%28by%20ref%29))
  (if (== (Utilities|GetClass OtherActor) "/Game/BP/BP_FirstLine.BP_FirstLine_C")
    (Rendering|Material|SetMaterial (Variables|Default|GetColor%20Plane) 0 "/Game/MATERIALS/MI_Square_White.MI_Square_White")
    (Rendering|SetVisibility (Variables|Default|GetBoxTrigger) false false)
    (Transformation|SetRelativeLocation (Variables|Default|GetBoxTrigger) "0, 0,-200.000000" false true)
    (Variables|/Script/Engine.PrimitiveComponent|SetbGenerateOverlapEvents (Variables|Default|GetBoxTrigger) false)))

(event Custom|RememberForReset
  (Variables|Default|SetRememberMaterial (Rendering|Material|GetMaterial (Variables|Default|GetColor%20Plane) 0))
  (Variables|Default|SetRememberVisibility (Variables|/Script/Engine.SceneComponent|GetbVisible (Variables|Default|GetBoxTrigger)))
  (Variables|Default|SetRememberLocation (Variables|/Script/Engine.SceneComponent|GetRelativeLocation (Variables|Default|GetBoxTrigger)))
  (Variables|Default|SetRememberIsOverlap (Variables|/Script/Engine.PrimitiveComponent|GetbGenerateOverlapEvents (Variables|Default|GetBoxTrigger))))

(event Custom|Move_Event
  (params (Move :type Enum_Direction%20Enum :default "NewEnumerator0"))
  (if (== (Variables|/Script/Engine.SceneComponent|GetbVisible (Variables|Default|GetLighted%20Plane)) true)
    (Rendering|SetVisibility (Variables|Default|GetLighted%20Plane) false false)))

(event EventBeginPlay
  (Ref|SetChunkRef)
  (Ref|SetPlayerControllerRef)
  (Ref|SetCharacterRef)
  (EventDispatchers|AssignMoveEvent (Variables|Ref|GetPlayerController_Ref) (EventDispatchers|CreateEvent :!event Custom|Move_Event))
  (CallFunction|RememberforReset))

(event Collision|EventActorBeginOverlap
  (params (OtherActor :type Actor%20Object%20Reference)))

(event EventTick
  (params (DeltaSeconds :type Float%20%28single-precision%29)))

(event EventLightSquare
  (Utilities|FlowControl|DelayUntilNextTick)
  (if (== (Variables|/Script/Engine.SceneComponent|GetbVisible (Variables|Default|GetLighted%20Plane)) false)
    (Rendering|SetVisibility (Variables|Default|GetLighted%20Plane) true false)))

(event EventPoolResetAble
  (Rendering|Material|SetMaterial (Variables|Default|GetColor%20Plane) 0 (Variables|Default|GetRememberMaterial))
  (Rendering|SetVisibility (Variables|Default|GetBoxTrigger) (Variables|Default|GetRememberVisibility) false)
  (Transformation|SetRelativeLocation (Variables|Default|GetBoxTrigger) (Variables|Default|GetRememberLocation) false true)
  (Variables|/Script/Engine.PrimitiveComponent|SetbGenerateOverlapEvents (Variables|Default|GetBoxTrigger) (Variables|Default|GetRememberIsOverlap)))

(fn ConstructionScript)

(fn SetPlayerControllerRef
  (Utilities|IsValid (Variables|Ref|GetPlayerController_Ref)
    (:Is%20Not%20Valid
      (bind _returnvalue (Actor|GetActorOfClass "/Game/BP/BP_PlayerController.BP_PlayerController_C"))
      (Variables|Ref|SetPlayerController_Ref _returnvalue))))

(fn SetCharacterRef
  (Utilities|IsValid (Variables|Ref|GetCharacter_Ref)
    (:Is%20Not%20Valid
      (bind _returnvalue (Actor|GetActorOfClass "/Game/BP/BP_Character.BP_Character_C"))
      (Variables|Ref|SetCharacter_Ref _returnvalue))))

(fn SetChunkRef
  (Utilities|IsValid (Variables|Ref|GetChunk_Ref)
    (:Is%20Not%20Valid
      (bind _returnvalue (Actor|GetActorOfClass "/Game/BP/BP_Chunk.BP_Chunk_C"))
      (Variables|Ref|SetChunk_Ref _returnvalue))))