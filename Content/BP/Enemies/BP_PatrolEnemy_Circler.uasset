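; Patrol enemy that steps in response to player moves, cycling through four movement offsets in order or at random.
; Each qualifying move eases it to the stored target via timeline, then picks the next one and line-traces to tell that square to light up.
; A block hit by the trace makes it skip movement next turn and re-pick.
; Overlapping the player deals damage, then blinks with collision off until the next move event.
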(event EventBeginPlay
  (|CallParentFunction)
  (Variables|Enemy|SetRememberMaterial (Rendering|Material|GetMaterial (Variables|Default|GetEnemyStaticMesh) 0)))

(event EventTick
  (params (DeltaSeconds :type Float%20%28single-precision%29)))

(event EventMoveEvent
  (params (Move :type Enum_Direction%20Enum :default "NewEnumerator0")))

(event EventEnemyMoveEvent
  (params (CharState :type Enum_CharacterStates%20Enum :default "NewEnumerator7"))
  (|CallParentFunction CharState)
  (Variables|Default|Set%20CharStateMoveEvent CharState)
  (switch Utilities|FlowControl|Switch|SwitchonEnum_CharacterStates (Variables|Default|Get%20CharStateMoveEvent)
    (:NewEnumerator0
      (Utilities|EnableCollisionBack))
    (:NewEnumerator2
      (Utilities|EnableCollisionBack :!label _label)
      (if (Variables|Default|GetFirstTurnNoTimeline_Flag)
        (Variables|move|SetEnemyLocation%20Old (.location (Transformation|GetActorTransform)) :!label _label_2)
        (Utilities|FlowControl|MultiGate (Variables|Enemy|GetisTurnsRandom) true -1
          (:Out%200
            (Utilities|SetEnemyLocationNew))
          (:Out%201
            (Utilities|SetEnemyLocationNew 1))
          (:Out%202
            (Utilities|SetEnemyLocationNew 2))
          (:Out%203
            (Utilities|SetEnemyLocationNew 3)))
        (bind (_outhit _returnvalue) (Collision|LineTraceForObjects (+ (Variables|move|GetEnemyLocation%20Old) "0,0,300.000000") (+ (Variables|Move|GetEnemyLocation%20New) "0,0,-25.000000") (Variables|Move|GetObject%20Types) false 0 "None" true "(R=1.000000,G=0.000000,B=0.000000,A=1.000000)" "(R=0.000000,G=1.000000,B=0.000000,A=1.000000)" 1.0))
        (if _returnvalue
          (if (Utilities|ClassIsChildOf (Utilities|GetClass (.HitActor (Collision|BreakHitResult _outhit))) "/Game/BP/Squares/BP_Square_Block.BP_Square_Block_C")
            (Variables|Default|SetFirstTurnNoTimeline_Flag true)
            (else
              (Class|BPIEnemyLightSquareAble|EnemyLightSquare(Message) (.HitActor (Collision|BreakHitResult _outhit)))
              (Variables|Default|SetFirstTurnNoTimeline_Flag false))))
        (else
          (bind _0_to_1 (Timeline|Timeline_EnemyMove PlayFromStart)
            (:Update
              (Transformation|SetActorLocationAndRotation (Math|Interpolation|Ease "EaseInOut" _0_to_1 (Variables|move|GetEnemyLocation%20Old) (Variables|Move|GetEnemyLocation%20New) 3.0) "0, 0, 0"))
            (:Finished
              (goto _label_2))))))
    (:NewEnumerator3
      (goto _label))
    (:NewEnumerator6
      (goto _label))))

(event EventCharacterOverlap
  (Utilities|FlowControl|FlipFlop
    (:A
      (Utilities|FlowControl|DoOnce false :!label _label
        (:Completed
          (Default|WriteChangeHealth (Variables|Default|GetCharacter_Ref) -10)
          (Rendering|Material|SetMaterial (Variables|Default|GetEnemyStaticMesh) 0 "/Game/MATERIALS/Enemy_Blinking.Enemy_Blinking")
          (Variables|Move|SetNextTurnFlag true)
          (Collision|SetActorEnableCollision false))))
    (:B
      (goto _label Reset))))

(fn ConstructionScript
  (|CallParentFunction))