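; Patrol enemy actor that reacts to player controller move and character patrol events through empty handler stubs, along with empty character overlap handlers.
; On BeginPlay it caches character, controller and enemy-character references, sets its text label and binds both events, retrying until the character is valid.
; Overlapping a grey line triggers a one-shot countdown on the text, switching to a blinking material at the final step before disabling, hiding and destroying itself.
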(event Custom|MoveEvent
  (params (Move :type Enum_Direction%20Enum :default "NewEnumerator0")))

(event Custom|EnemyCharOverlap)

(event Custom|CharacterOverlap)

(event Custom|PatrolMove
  (params (CharState :type Enum_CharacterStates%20Enum :default "NewEnumerator7")))

(event EventBeginPlay
  (ref|SetCharacterRef)
  (Ref|SetPlayerControllerRef)
  (Ref|SetEnemyCharacterRef)
  (Rendering|Components|TextRender|SetText (Variables|Default|GetTextRender) (Variables|DelayDestroy|GetTextName))
  (EventDispatchers|AssignMoveEvent (Variables|Ref|GetPlayerController_Ref) (EventDispatchers|CreateEvent :!event Custom|MoveEvent))
  (Utilities|IsCharacterRefValid
    (:true
      (EventDispatchers|AssignPatrolMove (Variables|ref|GetCharacter_Ref) (EventDispatchers|CreateEvent :!event Custom|PatrolMove)))))

(event Collision|EventActorBeginOverlap
  (params (OtherActor :type Actor%20Object%20Reference))
  (Utilities|ActorOverlapping OtherActor
    (:GreyLine
      (Utilities|FlowControl|DoOnce false
        (:Completed
          (Utilities|DelayDestroy 2 0.5
            (:Completed
              (Collision|SetActorEnableCollision false)
              (Rendering|SetActorHiddenInGame true)
              (Actor|DestroyActor))))))
    (:Character
      (CallFunction|CharacterOverlap))
    (:EnemyCharacter
      (CallFunction|EnemyCharOverlap))))

(event EventTick
  (params (DeltaSeconds :type Float%20%28single-precision%29)))

(fn ConstructionScript)

(fn SetCharacterRef
  (Utilities|IsValid (Variables|ref|GetCharacter_Ref)
    (:Is%20Not%20Valid
      (bind _returnvalue (Actor|GetActorOfClass "/Game/BP/BP_Character.BP_Character_C"))
      (Variables|ref|SetCharacter_Ref _returnvalue))))

(fn SetPlayerControllerRef
  (Utilities|IsValid (Variables|Ref|GetPlayerController_Ref)
    (:Is%20Not%20Valid
      (bind _returnvalue (Actor|GetActorOfClass "/Game/BP/BP_PlayerController.BP_PlayerController_C"))
      (Variables|Ref|SetPlayerController_Ref _returnvalue))))

(fn SetEnemyCharacterRef
  (Utilities|IsValid (Variables|Ref|GetEnemyCharacter_Ref)
    (:Is%20Not%20Valid
      (bind _returnvalue (Actor|GetActorOfClass "/Game/BP/BP_EnemyCharacter.BP_EnemyCharacter_C"))
      (Variables|Ref|SetEnemyCharacter_Ref _returnvalue))))