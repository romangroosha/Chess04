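; BP_FlyingStatusText is a short-lived actor that shows a status text widget in the world at a location taken from the player character.
; On BeginPlay it caches the BP_Character found by class lookup and teleports its widget component to that character's MoveLocationOld.
; It destroys itself after a fixed four-second delay, with no movement logic in its own graphs.
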(event EventBeginPlay
  (Ref|SetCharacterRef)
  (Transformation|SetWorldLocation (Variables|Default|GetWidgetComp) (Variables|/Game/BP/BP_Character.BP_Character_C|GetMove_Location_Old (Variables|Ref|GetCharacter_Ref)) false true)
  (Utilities|FlowControl|Delay 4.0)
  (Actor|DestroyActor))

(fn ConstructionScript)

(fn SetCharacterRef
  (Utilities|IsValid (Variables|Ref|GetCharacter_Ref)
    (:Is%20Not%20Valid
      (bind _returnvalue (Actor|GetActorOfClass "/Game/BP/BP_Character.BP_Character_C"))
      (Variables|Ref|SetCharacter_Ref _returnvalue))))